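; BPFL_Functions is a Blueprint function library of global shortcuts for the game's core framework objects.
; Getters cast the first player's character and controller, the game mode and the game instance to their project Blueprint classes.
; Show Mouse Cursor builds on the controller getter to toggle the cursor and switch between Game and UI input, with widget focus, and Game Only.
; Get Anim Instance is an empty stub.
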(fn GetPlayerBP
  (bind _asbp_character_base (Utilities|Casting|CastToBP_CharacterBase (Game|GetPlayerCharacter 0)))
  (return _asbp_character_base))

(fn GetPlayerControllerBP
  (bind _asbp_character_controller (Utilities|Casting|CastToBP_CharacterController (Game|GetPlayerController 0)))
  (return _asbp_character_controller))

(fn GetGameMode
  (bind _asbp_level_game_mode (Utilities|Casting|CastToBP_LevelGameMode (Game|GetGameMode)))
  (return _asbp_level_game_mode))

(fn GetAnimInstance)

(fn GetGameInstance
  (bind _asbp_game_instance (Utilities|Casting|CastToBP_GameInstance (Game|GetGameInstance)))
  (return _asbp_game_instance))

(fn ShowMouseCursor
  (params (Enabled :type Boolean) (Widget%20to%20focus :type User%20Widget%20Object%20Reference))
  (bind _bp_character_controller (CallFunction|GetPlayerControllerBP))
  (bind _output_get (Variables|/Script/Engine.PlayerController|SetbShowMouseCursor (CallFunction|GetPlayerControllerBP) Enabled))
  (if _output_get
    (Input|SetInputModeGameandUI _bp_character_controller Widget%20to%20focus "DoNotLock" true)
    (else
      (Input|SetInputModeGameOnly _bp_character_controller))))