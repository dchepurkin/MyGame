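; BP_StatSphere is a pickup orb that restores a fraction of a character's max health, mana or stamina, by Type.
; On authority it arcs to a random nearby point via timeline and obstacle traces, then enables collision, bobs and starts a despawn countdown.
; The outer collision locks onto the first overlapping character, starting accelerating homing on Tick.
; Inner collision with that target calls the server restore from the remote side and destroys the orb.
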(event OnComponentBeginOverlap(CollisionExternal)
  (params (OverlappedComponent :type Primitive%20Component%20Object%20Reference) (OtherActor :type Actor%20Object%20Reference) (OtherComp :type Primitive%20Component%20Object%20Reference) (OtherBodyIndex :type Integer) (bFromSweep :type Boolean) (SweepResult :type Hit%20Result%20Structure%20%28by%20ref%29))
  (bind _start_location (Variables|Default|GetStart%20Location))
  (Variables|Default|GetTarget
    (:then)
    (:else
      (bind _asbp_character_base (Utilities|Casting|CastToBP_CharacterBase OtherActor))
      (Variables|Default|SetTarget _asbp_character_base)
      (Components|DestroyComponent (Variables|Default|GetCollision%20External)) ; удаляем внешнюю колизию
      (Utilities|Time|ClearTimerbyFunctionName 0 "Destroy At Time") ; отключаем таймер
      (Utilities|FlowControl|Gate true) ; enters at Open
    )))

(event OnComponentBeginOverlap(CollisionInternal)
  (params (OverlappedComponent :type Primitive%20Component%20Object%20Reference) (OtherActor :type Actor%20Object%20Reference) (OtherComp :type Primitive%20Component%20Object%20Reference) (OtherBodyIndex :type Integer) (bFromSweep :type Boolean) (SweepResult :type Hit%20Result%20Structure%20%28by%20ref%29))
  (bind _target (Variables|Default|GetTarget))
  (bind _target_2 (Variables|Default|GetTarget))
  (bind _target_3 (Variables|Default|GetTarget))
  ;[1 1 1] Восстановление ресурсов
  (if (== OtherActor (Variables|Default|GetTarget))
    (Utilities|FlowControl|Sequence
      (:then_0
        (Networking|SwitchHasAuthority
          (:Remote
            (switch Utilities|FlowControl|Switch|SwitchonE_Stat (Variables|Default|GetType)
              (:NewEnumerator0
                (Default|RestoreHealthServer _target (* (Variables|/Game/PolygonDungeonOnline/Character/Blueprints/BP_CharacterBase.BP_CharacterBase_C|GetMax%20Health _target) (Variables|Default|GetDamage))))
              (:NewEnumerator1
                (Default|RestoreManaServer _target_3 (* (Variables|/Game/PolygonDungeonOnline/Character/Blueprints/BP_CharacterBase.BP_CharacterBase_C|GetMax%20Mana _target_3) (Variables|Default|GetDamage))))
              (:NewEnumerator2
                (Default|RestoreStaminaServer _target_2 (* (Variables|/Game/PolygonDungeonOnline/Character/Blueprints/BP_CharacterBase.BP_CharacterBase_C|GetMax%20Stamina _target_2) (Variables|Default|GetDamage))))))))
      (:then_1
        (Utilities|Time|ClearTimerbyFunctionName 0 "Increment Rotation Alpha")
        (Utilities|Time|ClearTimerbyFunctionName 0 "Increment Speed")
        (Rendering|SetActorHiddenInGame true))
      (:then_2
        (Actor|DestroyActor)))))

(event Custom|Animation
  (Collision|SetCollisionEnabled (Variables|Default|GetCollision%20External) "QueryAndPhysics") ; после  перелета сферы включаем колизии
  (Utilities|Time|SetTimerbyFunctionName 0 "Destroy At Time" 1.0 true) ; Запускаем таймер, по истечении которого сфера самоуничтожится
  (Variables|Default|SetStart%20Location (Transformation|GetActorLocation))
  ;[1 1 1] Анимация ливитирования сферы
  (bind _sphere_transform (Timeline|Sphere%20Transform PlayFromStart)
    (:Update
      (Transformation|SetActorLocation (Math|Vector|Lerp(Vector) (+ (Variables|Default|GetStart%20Location) "0.000000,0.000000,-10.000000") (+ (Variables|Default|GetStart%20Location) "0.000000,0.000000,10.000000") _sphere_transform) false false))))

(event EventBeginPlay
  (bind _returnvalue (Transformation|GetActorLocation))
  (bind _returnvalue_2 (Transformation|GetActorLocation))
  (bind _returnvalue_3 (Transformation|GetActorLocation))
  (bind _radius (Variables|Default|GetRadius))
  (bind (_x _y _z) (Math|Vector|BreakVector _returnvalue_3))
  (Networking|SwitchHasAuthority
    (:Authority
      (bind _output_get (Variables|Default|SetStart%20Location (Transformation|GetActorLocation))) ; Откуда вылетает сфера
      (bind _output_get_2 (Variables|Default|SetTarget%20Location (Math|Vector|MakeVector (.X (Math|Vector|BreakVector (Math|Random|RandomPointinBoundingBox _output_get (Math|Vector|MakeVector _radius _radius 1e+02)))) (.Y (Math|Vector|BreakVector (Math|Random|RandomPointinBoundingBox _output_get (Math|Vector|MakeVector _radius _radius 1e+02)))) (.Z (Math|Vector|BreakVector _output_get))))) ; Куда вылетает сфера
      (Transformation|SetActorRotation (Math|Rotator|FindLookatRotation (Variables|Default|GetStart%20Location) _output_get_2))
      ;[1 1 1] Меняем положение сферы от начальных координат к конечным через таймлайн
      (bind (_direction _position_xy _position_z) (Timeline|Start%20Animation Play)
        (:Update
          (Utilities|FlowControl|Sequence
            (:then_0
              (bind _returnvalue_4 (Collision|LineTraceByChannel _returnvalue_2 (+ _returnvalue_2 (* (Math|Vector|GetForwardVector (Transformation|GetActorRotation)) 5e+01)) "TraceTypeQuery1" false 0 "None")) ; Трасировка для проверки препятствий спереди относительно движения
              (if (not _returnvalue_4)
                (Transformation|SetActorLocation (Math|Vector|MakeVector (.x (Math|Vector|Lerp(Vector) (Variables|Default|GetStart%20Location) (Variables|Default|GetTarget%20Location) _position_xy)) (.y (Math|Vector|Lerp(Vector) (Variables|Default|GetStart%20Location) (Variables|Default|GetTarget%20Location) _position_xy)) (.z _returnvalue)) false false)))
            (:then_1
              (bind _returnvalue_5 (Collision|LineTraceByChannel _returnvalue_3 (Math|Vector|MakeVector _x _y (- _z 5e+01)) "TraceTypeQuery1" false 0 "None")) ; Трасировка для проверки препятствий спереди относительно движения
              (if _returnvalue_5
                (Utilities|FlowControl|Sequence
                  (:then_0
                    (Timeline|Start%20Animation Stop))
                  (:then_1
                    (CallFunction|Animation :!label _label)))
                (else
                  (Transformation|SetActorLocation (Math|Vector|MakeVector (.x _returnvalue) (.y _returnvalue) (Math|Float|Lerp (.Z (Math|Vector|BreakVector (Variables|Default|GetStart%20Location))) (+ (.Z (Math|Vector|BreakVector (Variables|Default|GetStart%20Location))) 2.5e+02) _position_z)) false false))))))
        (:Finished
          (goto _label))))
    (:Remote
      (Rendering|Material|SetMaterial (Variables|Default|GetSphere) 0 (Utilities|Select :Index (Variables|Default|GetType) :NewEnumerator0 (Variables|Default|GetHealth%20Material) :NewEnumerator1 (Variables|Default|GetMana%20Material) :NewEnumerator2 0)))))

(event EventTick
  (params (DeltaSeconds :type Float%20%28single-precision%29))
  (bind _start_location (Variables|Default|GetStart%20Location))
  (Utilities|FlowControl|Gate true
    (:Exit
      (Utilities|FlowControl|Sequence
        (:then_0
          ;[1 1 1] Анимация ливитирования сферы
          (bind _sphere_transform (Timeline|Sphere%20Transform Stop)
            (:Update
              (Transformation|SetActorLocation (Math|Vector|Lerp(Vector) (+ _start_location "0.000000,0.000000,-10.000000") (+ _start_location "0.000000,0.000000,10.000000") _sphere_transform) false false))))
        (:then_1
          ;[1 1 1] Поворот сферы за целью
          (Transformation|SetActorRotation (Math|Rotator|Lerp(Rotator) (Transformation|GetActorRotation) (Math|Rotator|FindLookatRotation (Transformation|GetActorLocation) (Transformation|GetActorLocation (Variables|Default|GetTarget))) (Variables|Default|GetAlpha) true))
          (Utilities|FlowControl|DoOnce false
            (:Completed
              (Utilities|Time|SetTimerbyFunctionName 0 "Increment Rotation Alpha" 0.1 true))))
        (:then_2
          ;[1 1 1] Перемещение сферы к цели
          (Transformation|AddActorWorldOffset (* (Math|Vector|GetForwardVector (Transformation|GetActorRotation)) (Variables|Default|GetSpeed)))
          (Utilities|FlowControl|DoOnce false
            (:Completed
              (Utilities|Time|SetTimerbyFunctionName 0 "Increment Speed" 0.02 true))))))))

(fn ConstructionScript)

(fn DestroyatTime
  (bind _result (Math|Float|DecrementFloat (Variables|Default|GetTime))
    (:%20%20
      (bind _output_get (Variables|Default|SetTime _result))
      (if (== _output_get 0.0)
        (Utilities|Time|ClearTimerbyFunctionName 0 "Destroy At Time")
        (Actor|DestroyActor)))))

(fn IncrementRotationAlpha
  (bind _output_get (Variables|Default|SetAlpha (+ (Variables|Default|GetAlpha) 0.01)))
  (if (> _output_get 1.0)
    (Variables|Default|SetAlpha 1.0)))

(fn IncrementSpeed
  (bind _output_get (Variables|Default|SetSpeed (+ (Variables|Default|GetSpeed) 0.15)))
  (if (> _output_get 1e+02)
    (Variables|Default|SetSpeed 1e+02)))