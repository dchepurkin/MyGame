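; BP_Switch is a lever switch item actor for the dungeon game, with a handle component that rotates as it is switched.
; Its Switch Item function takes an alpha and interpolates the handle's relative pitch between two fixed angles.
; The event graph and construction script add no logic of their own, so the alpha comes from outside this graph.
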(event EventBeginPlay
  (|CallParentFunction) ; This node is disabled and will not be called.\nDrag off pins to build functionality.
)

(event Collision|EventActorBeginOverlap
  (params (OtherActor :type Actor%20Object%20Reference))
  (|CallParentFunction OtherActor) ; This node is disabled and will not be called.\nDrag off pins to build functionality.
)

(event EventTick
  (params (DeltaSeconds :type Float%20%28single-precision%29))
  (|CallParentFunction DeltaSeconds) ; This node is disabled and will not be called.\nDrag off pins to build functionality.
)

(fn ConstructionScript
  (|CallParentFunction))

(fn SwitchItem
  (params (Alpha :type Float%20%28single-precision%29))
  (Transformation|SetRelativeRotation (Variables|Default|GetSwitchHandle) (Math|Rotator|Lerp(Rotator) "0, 0,-70.000000" "0, 0,40.000000" Alpha) false false))