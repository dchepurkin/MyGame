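; BP_Gates is a usable dungeon item for a gate that raises and lowers.
; Its SwitchItem override slides the Gate component vertically between two fixed relative heights, driven by the Alpha it receives.
; Its CanUse override adds a condition to the parent check: every entry in ItemsToOpen must be activated, so other items act as prerequisites for using the gate.
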(event EventBeginPlay
  (|CallParentFunction) ; This node is disabled and will not be called.\nDrag off pins to build functionality.
)

(event Collision|EventActorBeginOverlap
  (params (OtherActor :type Actor%20Object%20Reference)))

(event EventTick
  (params (DeltaSeconds :type Float%20%28single-precision%29)))

(fn ConstructionScript
  (|CallParentFunction))

(fn SwitchItem
  (params (Alpha :type Float%20%28single-precision%29))
  (Transformation|SetRelativeLocation (Variables|Default|GetGate) (Math|Vector|Lerp(Vector) "0, 0,250.000000" "0, 0,650.000000" Alpha) false false))

(fn CanUse
  (bind _array_element (Utilities|Array|ForEachLoopwithBreak (Variables|Default|GetItems%20To%20Open) :!label _label)
    (:LoopBody
      (if (not (Variables|/Game/PolygonDungeonOnline/Blueprints/Actors/Item/BP_Item_Base.BP_Item_Base_C|GetActivate _array_element))
        (LocalVariables|SetLocal%20Bool false)
        (goto _label Break)))
    (:Completed
      (return (and (|CallParentFunction) (LocalVariables|GetLocal%20Bool))))))