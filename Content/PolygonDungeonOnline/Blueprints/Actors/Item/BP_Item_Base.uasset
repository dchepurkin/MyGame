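; Base Blueprint for one-shot interactable items in a multiplayer dungeon, usable by living characters once their linked enemies and enemy groups are gone.
; The interaction box binds the overlapping character's use event and toggles its tooltip prompt.
; A successful use multicasts a timeline driving SwitchItem, an empty hook for children, while remotes also clear the custom-depth outline and play sound.
; Items already activated snap to their final state shortly after BeginPlay.
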(event OnComponentBeginOverlap(InterractiveBox)
  (params (OverlappedComponent :type Primitive%20Component%20Object%20Reference) (OtherActor :type Actor%20Object%20Reference) (OtherComp :type Primitive%20Component%20Object%20Reference) (OtherBodyIndex :type Integer) (bFromSweep :type Boolean) (SweepResult :type Hit%20Result%20Structure%20%28by%20ref%29))
  (bind _asbp_character_base (Utilities|Casting|CastToBP_CharacterBase OtherActor))
  (EventDispatchers|BindEventtoOnUseItem _asbp_character_base (EventDispatchers|CreateEvent :!event Custom|Use%20Item))
  (if (not (Variables|Default|GetActivate))
    (Default|CallOnInteractItem _asbp_character_base self (Variables|Default|GetToolTipMessage) true)))

(event OnComponentEndOverlap(InterractiveBox)
  (params (OverlappedComponent :type Primitive%20Component%20Object%20Reference) (OtherActor :type Actor%20Object%20Reference) (OtherComp :type Primitive%20Component%20Object%20Reference) (OtherBodyIndex :type Integer))
  (bind _asbp_character_base (Utilities|Casting|CastToBP_CharacterBase OtherActor))
  (EventDispatchers|UnbindallEventsfromOnUseItem _asbp_character_base)
  (if (not (Variables|Default|GetActivate))
    (Default|CallOnInteractItem _asbp_character_base self "" false)))

(event Custom|Use
  (bind _alpha (Timeline|UseItem_Timeline Play)
    (:Update
      (CallFunction|SwitchItem _alpha))))

(event Custom|Use%20Item
  (params (Character :type BP%20Character%20Base%20Object%20Reference))
  (if (not (Variables|Default|GetActivate))
    (if (not (Variables|/Game/PolygonDungeonOnline/Character/Blueprints/BP_CharacterBase.BP_CharacterBase_C|GetDead Character))
      (if (CallFunction|CanUse)
        (CallFunction|UseItemMulticast)
        (Variables|Default|SetActivate true)
        (else
          (Default|Message Character (Variables|Default|GetCantUseMessage))
          (CallFunction|CantUseItemSoundMulticast))))))

(event Custom|Use%20Item%20Multicast
  (Networking|SwitchHasAuthority
    (:Authority
      (CallFunction|Use :!label _label))
    (:Remote
      (Utilities|FlowControl|Sequence
        (:then_0
          (CallFunction|EnableOutline false)
          (goto _label))
        (:then_1
          (Audio|PlaySoundatLocation (Variables|Default|GetUseItemSound) (Transformation|GetActorLocation) "0, 0, 0" 1.0 1.0 0.0 0 0 0)
          (for _array_element (Collision|GetOverlappingActors (Variables|Default|GetInterractiveBox) "/Game/PolygonDungeonOnline/Character/Blueprints/BP_CharacterBase.BP_CharacterBase_C" :!class /Script/Engine.PrimitiveComponent)
            (bind _asbp_character_base (Utilities|Casting|CastToBP_CharacterBase _array_element))
            (Default|CallOnInteractItem _asbp_character_base self "" false)))))))

(event Custom|CantUseItemSound_Multicast
  (Audio|PlaySoundatLocation (Variables|Default|GetCantUseItemSound) (Transformation|GetActorLocation) "0, 0, 0" 1.0 1.0 0.0 0 0 0))

(event EventBeginPlay
  (Utilities|FlowControl|Delay 0.4)
  (if (Variables|Default|GetActivate)
    (CallFunction|SwitchItem 1.0)))

(fn ConstructionScript)

(fn CanUse
  (return (CallFunction|IsEnemysDead)))

(fn IsEnemysDead
  (if (> (Utilities|Array|Length (Variables|Default|GetEnemyGroops)) 0)
    (bind _array_element (Utilities|Array|ForEachLoopwithBreak (Variables|Default|GetEnemyGroops) :!label _label)
      (:LoopBody
        (Utilities|IsValid _array_element
          (:Is%20Valid
            (LocalVariables|SetLocal%20Bool false)
            (goto _label Break))))
      (:Completed
        _)))
  (if (> (Utilities|Array|Length (Variables|Default|GetEnemyes)) 0)
    (bind _array_element_2 (Utilities|Array|ForEachLoopwithBreak (Variables|Default|GetEnemyes) :!label _label_2)
      (:LoopBody
        (Utilities|IsValid _array_element_2
          (:Is%20Valid
            (LocalVariables|SetLocal%20Bool false)
            (goto _label_2 Break))))
      (:Completed
        _)))
  (return (LocalVariables|GetLocal%20Bool)))

(fn EnableOutline
  (params (Enabled :type Boolean))
  (for _array_element (Actor|GetComponentsbyTag "/Script/Engine.MeshComponent" "Outline")
    (Rendering|SetRenderCustomDepth _array_element Enabled)))

(fn SwitchItem
  (params (Alpha :type Float%20%28single-precision%29)))