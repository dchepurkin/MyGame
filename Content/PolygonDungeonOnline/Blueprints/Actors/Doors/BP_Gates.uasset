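; Gate door actor that slides upward to open, likely built on a shared door parent.
; Open takes an alpha and lerps the LeftDoor component's relative Z position between its lowered and raised heights.
; CanOpen gates this on every linked item in ItemsToOpen being activated and IsEnemysDead returning true.
; The event graph holds no active logic of its own.
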(event EventBeginPlay
  (|CallParentFunction) ; This node is disabled and will not be called.\nDrag off pins to build functionality.
)

(fn ConstructionScript
  (|CallParentFunction))

(fn Open
  (params (Alpha :type Float%20%28single-precision%29))
  (Transformation|SetRelativeLocation (Variables|Default|GetLeftDoor) (Math|Vector|Lerp(Vector) "0, 0,250.000000" "0, 0,650.000000" Alpha) false false))

(fn CanOpen
  (bind _array_element (Utilities|Array|ForEachLoopwithBreak (Variables|Default|GetItemsToOpen) :!label _label)
    (:LoopBody
      (if (not (Variables|/Game/PolygonDungeonOnline/Blueprints/Actors/Item/BP_Item_Base.BP_Item_Base_C|GetActivate _array_element))
        (LocalVariables|SetLocal%20Bool false)
        (goto _label Break)))
    (:Completed
      (return (and (LocalVariables|GetLocal%20Bool) (CallFunction|IsEnemysDead))))))