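; Server-authoritative enemy group actor that manages a set of enemy spawners as one encounter with shared aggro and reset.
; A looping Group Agro timer passes the first valid target found among members to any member without one.
; A death decrements the alive count and starts a once-gated timer that respawns dead members when no enemy has a target.
; The AmountOfEnemy RepNotify destroys the spawners and group when the count reaches zero.
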(event Custom|On%20Death
  (Networking|SwitchHasAuthority
    (:Authority
      (bind _result (Math|Integer|DecrementInt (Variables|Default|GetAmount%20Of%20Enemy))
        (:%20%20
          (Variables|Default|SetAmount%20Of%20Enemy _result)
          (Utilities|FlowControl|DoOnce false
            (:Completed
              (Utilities|Time|SetTimerbyFunctionName 0 "Check Enemyes Targets" 1.0 true))))))))

(event Custom|Reset%20Timer
  (Utilities|FlowControl|DoOnce false) ; enters at Reset
)

(event EventBeginPlay
  (Networking|SwitchHasAuthority
    (:Authority
      (Variables|Default|SetAmount%20Of%20Enemy (Utilities|Array|Length (Variables|Default|GetEnemy%20Spawners)))
      (for _array_element (Variables|Default|GetEnemy%20Spawners)
        (EventDispatchers|BindEventtoOnDeath _array_element (EventDispatchers|CreateEvent :!event Custom|On%20Death))
        (Utilities|Time|SetTimerbyFunctionName 0 "Group Agro" 1.0 true)))))

(fn ConstructionScript)

(fn OnRepAmountOfEnemy
  (Networking|SwitchHasAuthority
    (:Authority
      (if (== (Variables|Default|GetAmount%20Of%20Enemy) 0)
        (Utilities|Time|ClearTimerbyFunctionName 0 "Check Enemyes Targets")
        (Utilities|Time|ClearTimerbyFunctionName 0 "Group Agro")
        (for _array_element (Variables|Default|GetEnemy%20Spawners)
          (EventDispatchers|UnbindallEventsfromOnDeath _array_element)
          (Actor|DestroyActor _array_element))
        (Actor|DestroyActor)))))

(fn CheckEnemyesTargets
  (Networking|SwitchHasAuthority
    (:Authority
      (bind _array_element (Utilities|Array|ForEachLoopwithBreak (Variables|Default|GetEnemy%20Spawners))
        (:LoopBody
          (bind _enemy_character (Variables|/Game/PolygonDungeonOnline/Blueprints/Actors/Spawner/BP_SoloSpawner.BP_SoloSpawner_C|GetEnemy%20Character _array_element)
            (:then
              (Variables|/Game/PolygonDungeonOnline/Enemy/Blueprints/BP_Enemy.BP_Enemy_C|GetCurrent%20Target _enemy_character
                (:then
                  (LocalVariables|SetLocal%20Bool true))
                (:else)))
            (:else)))
        (:Completed
          (if (not (LocalVariables|GetLocal%20Bool))
            (Utilities|Time|ClearTimerbyFunctionName 0 "Check Enemyes Targets")
            (CallFunction|ResetTimer)
            (CallFunction|RespawnGroup)))))))

(fn RespawnGroup
  (Networking|SwitchHasAuthority
    (:Authority
      (for _array_element (Variables|Default|GetEnemy%20Spawners)
        (if (Variables|/Game/PolygonDungeonOnline/Blueprints/Actors/Spawner/BP_SoloSpawner.BP_SoloSpawner_C|GetDead _array_element)
          (Default|SpawnServer _array_element)))
      (Variables|Default|SetAmount%20Of%20Enemy (Utilities|Array|Length (Variables|Default|GetEnemy%20Spawners))))))

(fn GroupAgro
  (bind _enemy_spawners (Variables|Default|GetEnemy%20Spawners))
  (Networking|SwitchHasAuthority
    (:Authority
      (bind _array_element (Utilities|Array|ForEachLoopwithBreak _enemy_spawners :!label _label)
        (:LoopBody
          (bind _enemy_character (Variables|/Game/PolygonDungeonOnline/Blueprints/Actors/Spawner/BP_SoloSpawner.BP_SoloSpawner_C|GetEnemy%20Character _array_element)
            (:then
              (bind _current_target (Variables|/Game/PolygonDungeonOnline/Enemy/Blueprints/BP_Enemy.BP_Enemy_C|GetCurrent%20Target _enemy_character)
                (:then
                  (LocalVariables|SetTemp%20Target _current_target)
                  (goto _label Break))
                (:else)))
            (:else)))
        (:Completed
          (LocalVariables|GetTemp%20Target
            (:then
              (for _array_element_2 _enemy_spawners
                (bind _enemy_character_2 (Variables|/Game/PolygonDungeonOnline/Blueprints/Actors/Spawner/BP_SoloSpawner.BP_SoloSpawner_C|GetEnemy%20Character _array_element_2)
                  (:then
                    (Variables|/Game/PolygonDungeonOnline/Enemy/Blueprints/BP_Enemy.BP_Enemy_C|GetCurrent%20Target _enemy_character_2
                      (:then)
                      (:else
                        (Default|AgroServer _enemy_character_2 (LocalVariables|GetTemp%20Target)))))
                  (:else))))
            (:else)))))))