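; BP_SoloSpawner is a server-authoritative spawner that places a single enemy at its own transform on BeginPlay.
; It spawns a configurable controller and enemy class, has the controller possess the enemy, and listens to that enemy's OnDeath.
; On death it sets Dead and fires its own OnDeath dispatcher.
; It then unbinds and destroys itself unless flagged InGroup, in which case it stays alive.
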(event Custom|Spawn%20Server
  (Networking|SwitchHasAuthority
    (:Authority
      (bind _returnvalue (Game|SpawnActorfromClass (Variables|Default|GetController) (Math|Transform|MakeTransform "0, 0, 0" "0, 0, 0" "1,1,1") "Undefined" 0 0))
      (bind _returnvalue_2 (Game|SpawnActorfromClass (Variables|Default|GetEnemy) (Math|Transform|MakeTransform (Transformation|GetActorLocation) (Transformation|GetActorRotation) "1,1,1") "AdjustIfPossibleButAlwaysSpawn" 0 0))
      (bind _output_get (Variables|Default|SetEnemy%20Character _returnvalue_2))
      (Pawn|Possess _returnvalue _output_get)
      (EventDispatchers|BindEventtoOnDeath _returnvalue_2 (EventDispatchers|CreateEvent :!event Custom|On%20Death))
      (Variables|Default|SetDead false))))

(event Custom|On%20Death
  (Networking|SwitchHasAuthority
    (:Authority
      (Variables|Default|SetDead true)
      (Default|CallOnDeath)
      (if (not (Variables|Default|GetInGroup?))
        (EventDispatchers|UnbindallEventsfromOnDeath (Variables|Default|GetEnemy%20Character))
        (Actor|DestroyActor)))))

(event EventBeginPlay
  (Networking|SwitchHasAuthority
    (:Authority
      (CallFunction|SpawnServer))))

(fn ConstructionScript)