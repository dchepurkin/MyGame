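; Chat actor that owns the in-game chat window widget and relays input and messages to it.
; On BeginPlay it creates the widget, enables local player input, and binds to the player character's respawn event and the widget's send-message event.
; Enter opens the chat, while separate events close it or append a sender's message.
; The file shows no replication, so messages are only added to the local widget.
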(event Custom|Close%20Chat
  ;[1 1 1] Закрыть чат
  (Default|CloseChat (Variables|Default|GetChat%20Widget)))

(event Custom|Send%20Message
  (params (Sender :type Name) (Message%20Text :type Text))
  ;[1 1 1] Выводим сообщение в чат
  (Default|AddMessagetoChat (Variables|Default|GetChat%20Widget) Sender Message%20Text))

(event EventBeginPlay
  (bind _returnvalue (UserInterface|CreateWidget "/Game/PolygonDungeonOnline/UI/WBP_ChatWindow.WBP_ChatWindow_C" 0 (Variables|Default|GetMain%20HUD)))
  (bind _output_get (Variables|Default|SetChat%20Widget _returnvalue))
  (UserInterface|Viewport|AddtoViewport _output_get 0)
  (Input|EnableInput (Game|GetPlayerController 0))
  (bind _asbp_character_base (Utilities|Casting|CastToBP_CharacterBase (Game|GetPlayerCharacter 0)))
  (EventDispatchers|BindEventtoOnRespawn _asbp_character_base (EventDispatchers|CreateEvent :!event Custom|Close%20Chat))
  (EventDispatchers|BindEventtoOnSendMessage (Variables|Default|GetChat%20Widget) (EventDispatchers|CreateEvent _asbp_character_base :!event SendMessageServer)))

(event Input|KeyboardEvents|Enter
  (params (Key :type Key%20Structure :default "None"))
  ;[1 1 1] Открываем чат
  (:Pressed
    (Default|OpenChat (Variables|Default|GetChat%20Widget))))

(fn ConstructionScript)