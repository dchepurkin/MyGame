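; BP_StatSphere is a homing sphere actor that flies toward a character and destroys itself on close contact.
; An external-collision overlap stores the first BP_CharacterBase as Target and opens a Tick gate.
; Each tick it turns toward the target and moves forward frame-dependently, while Delay nodes pace capped ramps in turn alpha and speed.
; Any interior-collision overlap destroys it, with no stat logic here.
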(event OnComponentBeginOverlap(CollisionExternal)
  (params (OverlappedComponent :type Primitive%20Component%20Object%20Reference) (OtherActor :type Actor%20Object%20Reference) (OtherComp :type Primitive%20Component%20Object%20Reference) (OtherBodyIndex :type Integer) (bFromSweep :type Boolean) (SweepResult :type Hit%20Result%20Structure%20%28by%20ref%29))
  (Variables|Default|GetTarget
    (:then
      (Utilities|FlowControl|Gate true) ; enters at Open
    )
    (:else
      (bind _asbp_character_base (Utilities|Casting|CastToBP_CharacterBase OtherActor))
      (Variables|Default|SetTarget _asbp_character_base)
      (Utilities|FlowControl|Gate true) ; enters at Open
    )))

(event OnComponentBeginOverlap(CollisionInterior)
  (params (OverlappedComponent :type Primitive%20Component%20Object%20Reference) (OtherActor :type Actor%20Object%20Reference) (OtherComp :type Primitive%20Component%20Object%20Reference) (OtherBodyIndex :type Integer) (bFromSweep :type Boolean) (SweepResult :type Hit%20Result%20Structure%20%28by%20ref%29))
  (Actor|DestroyActor))

(event EventTick
  (params (DeltaSeconds :type Float%20%28single-precision%29))
  (Utilities|FlowControl|Gate true
    (:Exit
      (Utilities|FlowControl|Sequence
        (:then_0
          (Transformation|SetActorRotation (Math|Rotator|Lerp(Rotator) (Transformation|GetActorRotation) (Math|Rotator|FindLookatRotation (Transformation|GetActorLocation) (Transformation|GetActorLocation (Variables|Default|GetTarget))) (Variables|Default|GetAlpha) true))
          (Utilities|FlowControl|Delay 0.1)
          (bind _output_get (Variables|Default|SetAlpha (+ (Variables|Default|GetAlpha) 0.01)))
          (if (> _output_get 1.0)
            (Variables|Default|SetAlpha 1.0)))
        (:then_1
          (Transformation|AddActorWorldOffset (* (Math|Vector|GetForwardVector (Transformation|GetActorRotation)) (Variables|Default|GetSpeed)))
          (Utilities|FlowControl|Delay 0.1)
          (bind _output_get_2 (Variables|Default|SetSpeed (+ (Variables|Default|GetSpeed) 1.5)))
          (if (> _output_get_2 8e+01)
            (Variables|Default|SetSpeed 8e+01)))))))

(fn ConstructionScript)