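; BP_Chat handles the in-game text chat for the online dungeon game.
; On BeginPlay it creates the WBP_ChatWindow widget, enables input so Enter opens the chat, and binds an event to the local character's respawn.
; Messages pass from SendMessageOwn through SendMessageServer to SendMessageMulticast, which adds them to the chat window, with leftover debug prints along the way.
; A separate CloseChat event closes the window.
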(event Custom|Close%20Chat
  ;[1 1 1] Закрыть чат
  (Default|CloseChat (Variables|Default|GetChat%20Widget)))

(event Custom|Send%20Message%20Multicast
  (params (Character%20Name :type Name) (Message%20Text :type Text))
  ;[1 1 1] Отправляем сообщение всем игрокам
  (Development|PrintString "3")
  (Default|AddMessagetoChat (Variables|Default|GetChat%20Widget) Character%20Name Message%20Text))

(event Custom|Send%20Message%20Own
  (params (Character%20Name :type Name) (Message%20Text :type Text))
  ;[1 1 1] Отправляем сообщение всем игрокам
  (CallFunction|SendMessageServer Character%20Name Message%20Text))

(event Custom|Send%20Message%20Server
  (params (Character%20Name :type Name) (Message%20Text :type Text))
  ;[1 1 1] Отправляем сообщение всем игрокам
  (Development|PrintString "2")
  (CallFunction|SendMessageMulticast Character%20Name Message%20Text))

(event EventBeginPlay
  (bind _returnvalue (UserInterface|CreateWidget "/Game/PolygonDungeonOnline/UI/WBP_ChatWindow.WBP_ChatWindow_C" 0 (Variables|Default|GetMain%20HUD)))
  (bind _output_get (Variables|Default|SetChat%20Widget _returnvalue))
  (UserInterface|Viewport|AddtoViewport _output_get 0)
  (Input|EnableInput (Game|GetPlayerController 0))
  (bind _asbp_character_base (Utilities|Casting|CastToBP_CharacterBase (Game|GetPlayerCharacter 0)))
  (EventDispatchers|BindEventtoOnRespawn _asbp_character_base (EventDispatchers|CreateEvent :!event Custom|Close%20Chat)))

(event Input|KeyboardEvents|Enter
  (params (Key :type Key%20Structure :default "None"))
  ;[1 1 1] Открываем чат
  (:Pressed
    (Default|OpenChat (Variables|Default|GetChat%20Widget))))

(fn ConstructionScript)