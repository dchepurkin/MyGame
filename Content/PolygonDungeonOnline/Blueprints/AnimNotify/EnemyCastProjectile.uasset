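; Anim notify state that makes a ranged enemy cast a projectile during an animation.
; When the notify begins, it casts the mesh owner to BP_RangeEnemy and calls SpawnProjectile at the world transform of a named mesh socket.
; It passes the projectile class, damage, damage and buff radii, and buffs from its own variables, with the enemy's current target as the attack target.
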(fn ReceivedNotifyBegin
  (params (MeshComp :type Skeletal%20Mesh%20Component%20Object%20Reference) (Animation :type Anim%20Sequence%20Base%20Object%20Reference) (TotalDuration :type Float%20%28single-precision%29))
  (bind _asbp_range_enemy (Utilities|Casting|CastToBP_RangeEnemy (Components|GetOwner MeshComp)))
  (Default|SpawnProjectile _asbp_range_enemy (Variables|Default|GetProjectile%20Class) (Transformation|GetSocketTransform (Variables|/Script/Engine.Character|GetMesh _asbp_range_enemy) (Variables|Default|GetSocket%20Name) "RTS_World") (Variables|Default|GetDamage) (Variables|Default|GetDamage%20Radius) (Variables|Default|GetBuff%20Radius) (Variables|/Game/PolygonDungeonOnline/Enemy/Blueprints/BP_Enemy.BP_Enemy_C|GetCurrent%20Target _asbp_range_enemy) (Variables|Default|GetBuffs)))