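; Anim notify state for enemy melee attacks that uses a configured skill on the enemy's current target when it is within reach.
; On notify begin it constructs the Skill object on the BP_Enemy owner and runs TraceForDamage.
; That check sphere-overlaps an area in front of the enemy sized by its melee radius, then requires a clear Visibility line trace to the target before UseSkill fires.
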(fn ReceivedNotifyBegin
  (params (MeshComp :type Skeletal%20Mesh%20Component%20Object%20Reference) (Animation :type Anim%20Sequence%20Base%20Object%20Reference) (TotalDuration :type Float%20%28single-precision%29))
  (bind _asbp_enemy (Utilities|Casting|CastToBP_Enemy (Components|GetOwner MeshComp)))
  (bind _returnvalue (Game|ConstructObjectfromClass (Variables|Default|GetSkill) _asbp_enemy))
  (bind _can_damage (CallFunction|TraceforDamage _asbp_enemy (Variables|/Game/PolygonDungeonOnline/Enemy/Blueprints/BP_Enemy.BP_Enemy_C|GetCurrent%20Target _asbp_enemy)))
  (if _can_damage
    (Default|UseSkill _returnvalue (Utilities|Array|MakeArray (Variables|/Game/PolygonDungeonOnline/Enemy/Blueprints/BP_Enemy.BP_Enemy_C|GetCurrent%20Target _asbp_enemy)) _asbp_enemy)
    (return false)))

(fn TraceforDamage
  (params (Damager :type BP%20Enemy%20Object%20Reference) (Target :type BP%20Character%20Base%20Object%20Reference))
  (bind _returnvalue (Transformation|GetActorRotation Damager))
  (bind _returnvalue_2 (Transformation|GetActorLocation Damager))
  (bind _melee_atack_radius (Variables|/Game/PolygonDungeonOnline/Enemy/Blueprints/BP_Enemy.BP_Enemy_C|GetMelee%20Atack%20Radius Damager))
  (bind _returnvalue_3 (Math|Vector|GetForwardVector _returnvalue))
  (bind _returnvalue_4 (+ _melee_atack_radius 2e+01))
  (bind _returnvalue_5 (* _returnvalue_3 _returnvalue_4))
  (bind _returnvalue_6 (+ _returnvalue_2 _returnvalue_5))
  (bind _outhits (Collision|MultiSphereTraceForObjects Damager _returnvalue_6 _returnvalue_6 _melee_atack_radius (Utilities|Array|MakeArray "ObjectTypeQuery7") false 0 "None"))
  (bind _array_element (Utilities|Array|ForEachLoopwithBreak _outhits :!label _label)
    (:LoopBody
      (if (== Target (.HitActor (Collision|BreakHitResult _array_element)))
        (LocalVariables|SetLocal%20Bool true)
        (goto _label Break)))
    (:Completed
      (if (LocalVariables|GetLocal%20Bool)
        (bind _returnvalue_7 (Collision|LineTraceByChannel Damager (Transformation|GetActorLocation Damager) (Transformation|GetActorLocation Target) "TraceTypeQuery1" false 0 "None"))
        (if _returnvalue_7
          (return false)
          (else
            (return true)))
        (else
          (return false))))))