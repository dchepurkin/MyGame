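; Anim notify state that telegraphs an enemy's cone attack and applies a skill when the notify ends.
; Begin builds a procedural-mesh fan at foot level on the enemy's DamageArea from 5-degree trace endpoints, so walls don't clip it.
; End clears the mesh, then sweeps object line traces at 1-degree steps across the cone.
; Characters with an unblocked Visibility trace are collected uniquely and passed to a newly constructed Skill's UseSkill.
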(fn ReceivedNotifyBegin
  (params (MeshComp :type Skeletal%20Mesh%20Component%20Object%20Reference) (Animation :type Anim%20Sequence%20Base%20Object%20Reference) (TotalDuration :type Float%20%28single-precision%29))
  (bind _start_point (CallFunction|GetStartPoint MeshComp))
  (bind _asbp_enemy (Utilities|Casting|CastToBP_Enemy (Components|GetOwner MeshComp)))
  (LocalVariables|SetEnemy _asbp_enemy)
  (bind _hits_results (CallFunction|LineTraceforArea MeshComp))
  (for _index (range 0 (- (Utilities|Array|LastIndex _hits_results) 1))
    (LocalVariables|SetIndex _index)
    (Utilities|FlowControl|Sequence
      (:then_0
        (LocalVariables|SetL%20Point (.TraceEnd (Collision|BreakHitResult (Utilities|Array|Get(acopy) _hits_results (LocalVariables|GetIndex))))))
      (:then_1
        (LocalVariables|SetR%20Point (.TraceEnd (Collision|BreakHitResult (Utilities|Array|Get(acopy) _hits_results (+ (LocalVariables|GetIndex) 1))))))
      (:then_2
        (Class|ProceduralMeshComponent|CreateMeshSectionLinearColor (Variables|/Game/PolygonDungeonOnline/Enemy/Blueprints/BP_Enemy.BP_Enemy_C|GetDamageArea (LocalVariables|GetEnemy)) (LocalVariables|GetIndex) (Utilities|Array|MakeArray (- _start_point _start_point) (- (LocalVariables|GetL%20Point) _start_point) (- (LocalVariables|GetR%20Point) _start_point)) (Utilities|Array|MakeArray 0 2 1) 0 0 0 0 0 0 0 false)
        (Rendering|Material|SetMaterial (Variables|/Game/PolygonDungeonOnline/Enemy/Blueprints/BP_Enemy.BP_Enemy_C|GetDamageArea (LocalVariables|GetEnemy)) (LocalVariables|GetIndex) "/Game/PolygonDungeonOnline/Blueprints/Skill/EnemySkill/MI_SkillArea.MI_SkillArea"))))
  (Transformation|SetRelativeRotation (Variables|/Game/PolygonDungeonOnline/Enemy/Blueprints/BP_Enemy.BP_Enemy_C|GetDamageArea (LocalVariables|GetEnemy)) (* (Math|Rotator|MakeRotfromX (Transformation|GetActorForwardVector (LocalVariables|GetEnemy))) -1) false false))

(fn LineTraceforArea
  (params (Mesh%20Component :type Actor%20Component%20Object%20Reference))
  (bind _start_point (CallFunction|GetStartPoint Mesh%20Component))
  (for _index (range 0 (Math|Float|Truncate (/ (* (Variables|Default|GetHalfAngle) 2.0) 5.0)))
    (bind _outhit (Collision|LineTraceByChannel Mesh%20Component _start_point (+ _start_point (* (Math|Vector|RotateVectorAroundAxis (Transformation|GetActorForwardVector (Components|GetOwner Mesh%20Component)) (+ (* 5 (Math|Conversions|ToFloat(Integer) _index)) (* (Variables|Default|GetHalfAngle) -1.0)) "0, 0,1.000000") (Variables|Default|GetRadius))) "TraceTypeQuery1" false 0 "None"))
    (Utilities|Array|Add (LocalVariables|GetHits) _outhit))
  (return (LocalVariables|GetHits)))

(fn ReceivedNotifyEnd
  (params (MeshComp :type Skeletal%20Mesh%20Component%20Object%20Reference) (Animation :type Anim%20Sequence%20Base%20Object%20Reference))
  (bind _asbp_enemy (Utilities|Casting|CastToBP_Enemy (Components|GetOwner MeshComp)))
  (Class|ProceduralMeshComponent|ClearAllMeshSections (Variables|/Game/PolygonDungeonOnline/Enemy/Blueprints/BP_Enemy.BP_Enemy_C|GetDamageArea _asbp_enemy))
  (bind _returnvalue (Game|ConstructObjectfromClass (Variables|Default|GetSkill) _asbp_enemy))
  (bind _characters (CallFunction|LineTraceforDamage MeshComp))
  (Default|UseSkill _returnvalue _characters _asbp_enemy)
  (return false))

(fn GetStartPoint
  (params (Mesh%20Component :type Actor%20Component%20Object%20Reference))
  (bind _returnvalue (Components|GetOwner Mesh%20Component))
  (bind _returnvalue_2 (Transformation|GetActorLocation _returnvalue))
  (bind (_x _y _z) (Math|Vector|BreakVector _returnvalue_2))
  (return (Math|Vector|MakeVector _x _y (- _z (Variables|/Script/Engine.CapsuleComponent|GetCapsuleHalfHeight (Variables|/Script/Engine.Character|GetCapsuleComponent (.AsBP%20Enemy (Utilities|Casting|CastToBP_Enemy _returnvalue))))))))

(fn LineTraceforDamage
  (params (Mesh%20Component :type Mesh%20Component%20Object%20Reference))
  (bind _returnvalue (Components|GetOwner Mesh%20Component))
  (bind _returnvalue_2 (Transformation|GetActorLocation _returnvalue))
  (for _index (range 0 (Math|Float|Truncate (* (Variables|Default|GetHalfAngle) 2.0)))
    (bind _outhits (Class|KismetSystemLibrary|LineTraceMultiforObjects Mesh%20Component _returnvalue_2 (+ _returnvalue_2 (* (Math|Vector|RotateVectorAroundAxis (Transformation|GetActorForwardVector _returnvalue) (+ (Math|Conversions|ToFloat(Integer) _index) (* (Variables|Default|GetHalfAngle) -1.0)) "0, 0,1.000000") (Variables|Default|GetRadius))) (Utilities|Array|MakeArray "ObjectTypeQuery7") false 0 "None" true))
    (for _array_element _outhits
      (if (.bBlockingHit (Collision|BreakHitResult _array_element))
        (bind _returnvalue_3 (Collision|LineTraceByChannel Mesh%20Component (.TraceStart (Collision|BreakHitResult _array_element)) (.Location (Collision|BreakHitResult _array_element)) "TraceTypeQuery1" false 0 "None"))
        (if (not _returnvalue_3)
          (bind _asbp_character_base (Utilities|Casting|CastToBP_CharacterBase (.HitActor (Collision|BreakHitResult _array_element))))
          (Utilities|Array|AddUnique (LocalVariables|GetTemp%20Characters) _asbp_character_base)))))
  (return (LocalVariables|GetTemp%20Characters)))