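; Anim notify state that plays surface-specific footstep sounds for characters.
; On notify begin, it runs a short downward Visibility trace from a configurable socket on the mesh, ignoring the owning BP_CharacterBase.
; The hit physical material's surface type selects the Ground, Grass, Wood or Sand sound.
; PlayStepSound then plays it at the socket location with shared footstep attenuation.
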(fn ReceivedNotifyBegin
  (params (MeshComp :type Skeletal%20Mesh%20Component%20Object%20Reference) (Animation :type Anim%20Sequence%20Base%20Object%20Reference) (TotalDuration :type Float%20%28single-precision%29))
  (bind _socket_name (Variables|Default|GetSocket%20Name))
  (bind _returnvalue (Transformation|GetSocketLocation MeshComp _socket_name))
  (bind (_outhit _returnvalue_2) (Collision|LineTraceByChannel MeshComp _returnvalue (- _returnvalue "0, 0,100.000000") "TraceTypeQuery1" false (Utilities|Array|MakeArray (.AsBP%20Character%20Base (Utilities|Casting|CastToBP_CharacterBase (Components|GetOwner MeshComp)))) "None"))
  (if _returnvalue_2
    (switch Utilities|FlowControl|Switch|SwitchonEPhysicalSurface (Variables|/Script/PhysicsCore.PhysicalMaterial|GetSurfaceType (.PhysMat (Collision|BreakHitResult _outhit)))
      (:SurfaceType1
        (CallFunction|PlayStepSound MeshComp "/Game/PolygonDungeonOnline/Sounds/Steps/GROUND/Ground_Footsteps.Ground_Footsteps"))
      (:SurfaceType2
        (CallFunction|PlayStepSound MeshComp "/Game/PolygonDungeonOnline/Sounds/Steps/GRASS/Grass_Footsteps.Grass_Footsteps"))
      (:SurfaceType3
        (CallFunction|PlayStepSound MeshComp "/Game/PolygonDungeonOnline/Sounds/Steps/WOOD/Wood_Footsteps.Wood_Footsteps"))
      (:SurfaceType4
        (CallFunction|PlayStepSound MeshComp "/Game/PolygonDungeonOnline/Sounds/Steps/SAND/Sand_Footsteps.Sand_Footsteps")))))

(fn PlayStepSound
  (params (Mesh :type Skeletal%20Mesh%20Component%20Object%20Reference) (Sound :type Sound%20Cue%20Object%20Reference))
  (Audio|PlaySoundatLocation Mesh Sound (Transformation|GetSocketLocation Mesh (Variables|Default|GetSocket%20Name)) "0, 0, 0" 1.0 1.0 0.0 "/Game/PolygonDungeonOnline/Sounds/Steps/StepsAttenuation.StepsAttenuation" 0 0))