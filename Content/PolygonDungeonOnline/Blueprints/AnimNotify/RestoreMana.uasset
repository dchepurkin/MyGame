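; RestoreMana is an animation notify state that restores a character's mana when a combo hit requirement is met.
; On notify begin, it casts the mesh owner to BP_CharacterBase and checks that CurrentComboHits exactly equals ComboHitsNeed.
; On a match, it calls RestoreManaServer with MaxMana multiplied by RestoredMana, so the amount scales with the character's maximum mana.
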(fn ReceivedNotifyBegin
  (params (MeshComp :type Skeletal%20Mesh%20Component%20Object%20Reference) (Animation :type Anim%20Sequence%20Base%20Object%20Reference) (TotalDuration :type Float%20%28single-precision%29))
  (bind _asbp_character_base (Utilities|Casting|CastToBP_CharacterBase (Components|GetOwner MeshComp)))
  (if (== (Variables|/Game/PolygonDungeonOnline/Character/Blueprints/BP_CharacterBase.BP_CharacterBase_C|GetCurrent%20Combo%20Hits _asbp_character_base) (Variables|Default|GetCombo%20Hits%20Need))
    (Default|RestoreManaServer _asbp_character_base (* (Variables|/Game/PolygonDungeonOnline/Character/Blueprints/BP_CharacterBase.BP_CharacterBase_C|GetMax%20Mana _asbp_character_base) (Variables|Default|GetRestored%20Mana)))
    (return false)))