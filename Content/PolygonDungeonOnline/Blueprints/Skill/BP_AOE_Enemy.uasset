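; Enemy area-of-effect skill actor that damages and applies buffs to player-side characters, shown with a translucent red color.
; MakeDamage runs only on the server and handles the enemy-target case.
; It applies full radial damage scaled by the caster's OutputDamageGain, ignoring all BP_Enemy actors.
; It then applies each configured buff to every BP_CharacterBase overlapping the AOE component.
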(event EventBeginPlay
  (|CallParentFunction))

(event Collision|EventActorBeginOverlap
  (params (OtherActor :type Actor%20Object%20Reference)))

(event EventTick
  (params (DeltaSeconds :type Float%20%28single-precision%29)))

(fn ConstructionScript
  (|CallParentFunction))

(fn GetColor
  (return "(R=1.000000,G=0.000000,B=0.000000,A=0.047059)"))

(fn MakeDamage
  (bind _caster (Variables|Default|GetCaster))
  (bind _asbp_enemy (Utilities|Casting|CastToBP_Enemy _caster))
  (Networking|SwitchHasAuthority
    (:Authority
      (switch Utilities|FlowControl|Switch|SwitchonESkillTarget (Variables|Default|GetTarget)
        (:NewEnumerator1
          (bind _outactors (Actor|GetAllActorsOfClass "/Game/PolygonDungeonOnline/Enemy/Blueprints/BP_Enemy.BP_Enemy_C"))
          (Game|Damage|ApplyRadialDamage (* (Variables|Default|GetDamage) (Variables|/Game/PolygonDungeonOnline/Enemy/Blueprints/BP_Enemy.BP_Enemy_C|GetOutput%20Damage%20Gain%20%25 _asbp_enemy)) (Transformation|GetActorLocation) (Variables|Default|GetRadius) 0 _outactors _asbp_enemy 0 true "ECC_Visibility")
          (for _array_element (Collision|GetOverlappingActors (Variables|Default|GetAOE) "/Game/PolygonDungeonOnline/Character/Blueprints/BP_CharacterBase.BP_CharacterBase_C" :!class /Script/Engine.PrimitiveComponent)
            (bind _asbp_character_base (Utilities|Casting|CastToBP_CharacterBase _array_element))
            (for _array_element_2 (Variables|Default|GetBuffs)
              (Default|ApplyBuff _asbp_character_base (Variables|Default|GetCaster) _array_element_2))))))))