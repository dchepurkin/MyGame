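; BP_AOE_Skill is an area-of-effect skill Blueprint that starts by spawning an area actor at the player.
; Initialize shows the mouse cursor and spawns BP_AOE_Area at player character 0's location, owned by that character and sized by SkillRadius.
; SetTarget and IsTargetAvailable always return true, so no target is stored or checked here.
; The parent Initialize call is present but unconnected, so it never runs.
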(fn ConstructionScript
  (|CallParentFunction))

(fn SetTarget
  (params (Cast%20Target :type Character%20Object%20Reference))
  (return true))

(fn IsTargetAvailable
  (return true))

(fn Initialize
  (bind _returnvalue (Game|GetPlayerCharacter 0))
  (Variables|/Script/Engine.PlayerController|SetbShowMouseCursor (Game|GetPlayerController 0) true)
  (Game|SpawnActorfromClass "/Game/PolygonDungeonOnline/Blueprints/Actors/BP_AOE_Area.BP_AOE_Area_C" (Math|Transform|MakeTransform (Transformation|GetActorLocation _returnvalue) "0, 0, 0" "1,1,1") "AlwaysSpawn" _returnvalue (Variables|Default|GetSkill%20Radius) 0))