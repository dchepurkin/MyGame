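; Homing projectile for ranged skills that chases AttackTarget and applies damage and buffs when it overlaps it.
; The server handles steering and collision, choosing the target channel by whether the caster is a BP_CharacterBase.
; Area effects use a capsule trace filtered by line of sight, though buff areas use DamageRadius despite checking BuffRadius.
; It is destroyed on hit or impact, playing sound and FX and requesting camera shake for a character caster.
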(event OnComponentHit(Collision)
  (params (HitComponent :type Primitive%20Component%20Object%20Reference) (OtherActor :type Actor%20Object%20Reference) (OtherComp :type Primitive%20Component%20Object%20Reference) (NormalImpulse :type Vector :default "0, 0, 0") (Hit :type Hit%20Result%20Structure%20%28by%20ref%29))
  (Actor|DestroyActor))

(event OnComponentBeginOverlap(Collision)
  (params (OverlappedComponent :type Primitive%20Component%20Object%20Reference) (OtherActor :type Actor%20Object%20Reference) (OtherComp :type Primitive%20Component%20Object%20Reference) (OtherBodyIndex :type Integer) (bFromSweep :type Boolean) (SweepResult :type Hit%20Result%20Structure%20%28by%20ref%29))
  (if (== OtherActor (Variables|RangeProjectile|GetAttack%20Target))
    (CallFunction|MakeDamage)
    (CallFunction|CastBuffs)
    (Actor|DestroyActor)))

(event EventDestroyed
  (CallFunction|OnDestroy))

(event EventBeginPlay
  (Utilities|FlowControl|Delay 0.05)
  (Networking|SwitchHasAuthority
    (:Authority
      (Collision|SetCollisionEnabled (Variables|Default|GetCollision) "QueryAndPhysics")
      (Collision|SetCollisionResponsetoChannel (Variables|Default|GetCollision) (select (.bSuccess (Utilities|Casting|CastToBP_CharacterBase (Variables|RangeProjectile|GetCaster))) "ECC_GameTraceChannel2" "ECC_GameTraceChannel1") "ECR_Overlap"))
    (:Remote
      (Audio|PlaySoundatLocation (Variables|RangeProjectile|GetSpawn%20Sound) (Transformation|GetActorLocation) "0, 0, 0" 1.0 1.0 0.0 0 0 0))))

(event EventTick
  (params (DeltaSeconds :type Float%20%28single-precision%29))
  (bind _movement (Variables|Default|GetMovement))
  (Networking|SwitchHasAuthority
    (:Authority
      (bind _attack_target (Variables|RangeProjectile|GetAttack%20Target)
        (:then
          (Transformation|SetActorRotation (Math|Rotator|FindLookatRotation (Transformation|GetActorLocation) (Transformation|GetActorLocation _attack_target)))
          (Variables|/Script/Engine.MovementComponent|SetVelocity _movement (* (Math|Vector|GetForwardVector (Math|Rotator|FindLookatRotation (Transformation|GetActorLocation) (Transformation|GetActorLocation _attack_target))) (Variables|/Script/Engine.ProjectileMovementComponent|GetInitialSpeed _movement))))
        (:else)))))

(fn ConstructionScript)

(fn MakeDamage
  (bind _attack_target (Variables|RangeProjectile|GetAttack%20Target))
  (if (!= (Variables|RangeProjectile|GetDamage%20Radius) 0.0) ; если радиус 0 то только на цель
    (bind _output_get (LocalVariables|SetTargets (CallFunction|GetTargetsinArea (Transformation|GetActorLocation _attack_target) (Variables|RangeProjectile|GetDamage%20Radius))))
    (for _array_element _output_get
      (Game|Damage|ApplyDamage _array_element (Variables|RangeProjectile|GetDamage) 0 (Variables|RangeProjectile|GetCaster)))
    (else
      (Game|Damage|ApplyDamage _attack_target (Variables|RangeProjectile|GetDamage) 0 (Variables|RangeProjectile|GetCaster)))))

(fn CastBuffs
  (if (Math|Conversions|ToBoolean(Integer) (Utilities|Array|Length (Variables|RangeProjectile|GetBuffs)))
    (if (!= (Variables|RangeProjectile|GetBuff%20Radius) 0.0) ; если радиус 0 то только на цель
      (bind _output_get (LocalVariables|SetTargets (CallFunction|GetTargetsinArea (Transformation|GetActorLocation (Variables|RangeProjectile|GetAttack%20Target)) (Variables|RangeProjectile|GetDamage%20Radius))))
      (for _array_element _output_get
        (for _array_element_2 (Variables|RangeProjectile|GetBuffs)
          (Class|BPIBuff|ApplyBuff(Message) _array_element (Variables|RangeProjectile|GetCaster) _array_element_2)))
      (else
        (for _array_element_3 (Variables|RangeProjectile|GetBuffs)
          (Class|BPIBuff|ApplyBuff(Message) (Variables|RangeProjectile|GetAttack%20Target) (Variables|RangeProjectile|GetCaster) _array_element_3))))))

(fn OnDestroy
  (Utilities|FlowControl|Sequence
    (:then_0
      (Networking|SwitchHasAuthority
        (:Authority
          (bind _asbp_character_base (Utilities|Casting|CastToBP_CharacterBase (Variables|RangeProjectile|GetCaster)))
          (Default|CameraShakeServer _asbp_character_base (Variables|RangeProjectile|GetShake)))))
    (:then_1
      (Audio|PlaySoundatLocation (Variables|RangeProjectile|GetDestroy%20Sound) (Transformation|GetActorLocation) "0, 0, 0" 1.0 1.0 0.0 0 0 0)
      (bind _destroy_fx (Variables|RangeProjectile|GetDestroy%20FX)
        (:then
          (Effects|SpawnEmitteratLocation _destroy_fx (Transformation|GetActorLocation)))
        (:else)))))

(fn GetTargetsinArea
  (params (Point :type Vector) (Radius :type Float%20%28single-precision%29))
  (bind (_outhits _returnvalue) (Class|KismetSystemLibrary|CapsuleTraceMultiforObjects Point Point Radius 0.0 (Utilities|Array|MakeArray (select (.bSuccess (Utilities|Casting|CastToBP_CharacterBase (Variables|RangeProjectile|GetCaster))) "ObjectTypeQuery8" "ObjectTypeQuery7")) false 0 "None" false))
  (if _returnvalue
    (for _array_element _outhits
      (bind _returnvalue_2 (Collision|LineTraceByChannel (Transformation|GetActorLocation (Variables|RangeProjectile|GetAttack%20Target)) (Transformation|GetActorLocation (.HitActor (Collision|BreakHitResult _array_element))) "TraceTypeQuery1" false 0 "None" false))
      (if (not _returnvalue_2)
        (bind _ascharacter (Utilities|Casting|CastToCharacter (.HitActor (Collision|BreakHitResult _array_element))))
        (Utilities|Array|AddUnique (LocalVariables|GetLocal%20Targets) _ascharacter)))
    (return (LocalVariables|GetLocal%20Targets))
    (else
      (return (LocalVariables|GetLocal%20Targets)))))