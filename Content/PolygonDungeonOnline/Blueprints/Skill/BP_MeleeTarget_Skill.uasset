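; Targeted melee skill that either heals a friendly character or damages an enemy, then applies its buffs.
; Target type drives validation and execution: friendly casts fall back to the caster, invalid targets are rejected, and the caster turns toward others.
; On skill end, damage requires a range check and gates enemy buffs, while heals always apply.
; Separate skill and buff radii switch each effect from single-target to area around the target.
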(fn ConstructionScript
  (|CallParentFunction))

(fn IsTargetAvailable
  (if (|CallParentFunction)
    (switch Utilities|FlowControl|Switch|SwitchonESkillTarget (Variables|Default|GetTarget)
      (:NewEnumerator0
        (bind _asbp_character_base (Utilities|Casting|CastToBP_CharacterBase (Variables|Default|GetCast%20Target)))
        (if (Variables|/Game/PolygonDungeonOnline/Character/Blueprints/BP_CharacterBase.BP_CharacterBase_C|GetIsDead _asbp_character_base)
          (Default|CallOnScreenMessage (Variables|Default|GetCaster) "Цель мертва")
          (return false)
          (else
            (return true))))
      (:NewEnumerator1
        (Utilities|Casting|CastToBP_Enemy (Variables|Default|GetCast%20Target)
          (:then
            (return true))
          (:CastFailed
            (return false)))))
    (else
      (return false))))

(fn SetTarget
  (params (Cast%20Target :type Character%20Object%20Reference))
  (bind _caster (Variables|Default|GetCaster))
  (switch Utilities|FlowControl|Switch|SwitchonESkillTarget (Variables|Default|GetTarget)
    (:NewEnumerator0
      (bind _asbp_character_base (Utilities|Casting|CastToBP_CharacterBase Cast%20Target)
        (:then
          (Variables|Default|SetCast%20Target _asbp_character_base))
        (:CastFailed
          (Variables|Default|SetCast%20Target (Variables|Default|GetCaster))))
      (return true))
    (:NewEnumerator1
      (bind _asbp_enemy (Utilities|Casting|CastToBP_Enemy Cast%20Target)
        (:then
          (Variables|Default|SetCast%20Target _asbp_enemy)
          (return true))
        (:CastFailed
          (Utilities|Casting|CastToBP_CharacterBase Cast%20Target
            (:then
              (Default|CallOnScreenMessage _caster "Неподходящая цель"))
            (:CastFailed
              (Default|CallOnScreenMessage _caster "Нет цели")))
          (return false))))))

(fn Initialize
  (bind _caster (Variables|Default|GetCaster))
  (bind _cast_target (Variables|Default|GetCast%20Target))
  (switch Utilities|FlowControl|Switch|SwitchonESkillTarget (Variables|Default|GetTarget)
    (:NewEnumerator0
      (if (== _caster _cast_target)
        _
        (else
          (Default|LooktoTargertServer _caster _cast_target :!label _label))))
    (:NewEnumerator1
      (goto _label)))
  (|CallParentFunction))

(fn ApplyDamage
  (bind _caster (Variables|Default|GetCaster))
  (bind _cast_target (Variables|Default|GetCast%20Target))
  (if (Default|CanDamageTarget? (Variables|Default|GetCaster) (Variables|Default|GetCast%20Target) (/ (Variables|Default|GetMin%20Distance) 2.0))
    (if (!= (Variables|Default|GetSkill%20Radius) 0.0) ; если радиус 0 то только на цель
      (for _array_element (.Enemy (Default|LineTraceArea _caster (Transformation|GetActorLocation _cast_target) (Variables|Default|GetSkill%20Radius)))
        (Default|ApplyDamageServer _caster _array_element (Variables|Default|GetDamage) _caster))
      (else
        (Default|ApplyDamageServer _caster _cast_target (Variables|Default|GetDamage) _caster)))
    (return true)
    (else
      (return false))))

(fn ApplyHeal
  (if (!= (Variables|Default|GetSkill%20Radius) 0.0) ; если радиус 0 то только на цель
    (for _array_element (.Friendly (Default|LineTraceArea (Variables|Default|GetCaster) (Transformation|GetActorLocation (Variables|Default|GetCast%20Target)) (Variables|Default|GetSkill%20Radius)))
      (Class|BPIBuff|RestoreHealthSkill(Message) (Variables|Default|GetCaster) _array_element (Variables|Default|GetDamage)))
    (else
      (Class|BPIBuff|RestoreHealthSkill(Message) (Variables|Default|GetCaster) (Variables|Default|GetCast%20Target) (Variables|Default|GetDamage)))))

(fn EndSkill
  (switch Utilities|FlowControl|Switch|SwitchonESkillTarget (Variables|Default|GetTarget)
    (:NewEnumerator0
      (CallFunction|ApplyHeal)
      (CallFunction|ApplyBuffs :!label _label))
    (:NewEnumerator1
      (bind _success (CallFunction|ApplyDamage))
      (if _success
        (goto _label)))))

(fn ApplyBuffs
  (bind _caster (Variables|Default|GetCaster))
  (bind _caster_2 (Variables|Default|GetCaster))
  (bind _cast_target (Variables|Default|GetCast%20Target))
  (bind _caster_3 (Variables|Default|GetCaster))
  (bind _buff_radius (Variables|Default|GetBuff%20Radius))
  (bind _returnvalue (Transformation|GetActorLocation _cast_target))
  (bind (_enemy _friendly) (Default|LineTraceArea _caster_3 _returnvalue _buff_radius))
  ;[1 1 1] Вешаем баффы на все цели
  (if (Math|Conversions|ToBoolean(Integer) (Utilities|Array|Length (Variables|Default|GetBuff)))
    (for _array_element (Variables|Default|GetBuff)
      (if (!= (Variables|Default|GetBuff%20Radius) 0.0) ; Если радиус 0 то баф только на цель
        (for _array_element_2 (Utilities|Select :Index (Variables|Default|GetTarget) :NewEnumerator0 _friendly :NewEnumerator1 _enemy)
          (Class|BPIBuff|ApplyBufftoTarget(Message) _caster_2 _array_element_2 _caster_2 _array_element))
        (else
          (Class|BPIBuff|ApplyBufftoTarget(Message) _caster (Variables|Default|GetCast%20Target) _caster _array_element))))))