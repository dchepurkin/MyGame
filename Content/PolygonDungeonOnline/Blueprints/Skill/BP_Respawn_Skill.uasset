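; BP_Respawn_Skill is a respawn skill Blueprint that handles targeting of dead characters.
; Set Target stores only BP_CharacterBase targets and shows the caster an on-screen "unsuitable target" message in Russian for anything else, including enemies.
; IsTargetAvailable passes only when the stored target is valid and dead, telling the caster when the target is still alive.
; The respawn effect itself is not defined in these graphs.
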(fn SetTarget
  (params (Cast%20Target :type Character%20Object%20Reference))
  (bind _caster (Variables|Default|GetCaster))
  (bind _asbp_character_base (Utilities|Casting|CastToBP_CharacterBase Cast%20Target)
    (:then
      (Variables|Default|SetCast%20Target _asbp_character_base))
    (:CastFailed
      (Utilities|Casting|CastToBP_Enemy Cast%20Target
        (:then
          (Default|CallOnScreenMessage _caster "Неподходящая цель"))
        (:CastFailed
          (Default|CallOnScreenMessage _caster "Неподходящая цель"))))))

(fn IsTargetAvailable
  (bind _cast_target (Variables|Default|GetCast%20Target)
    (:then
      (bind _asbp_character_base (Utilities|Casting|CastToBP_CharacterBase _cast_target))
      (if (Variables|/Game/PolygonDungeonOnline/Character/Blueprints/BP_CharacterBase.BP_CharacterBase_C|GetIsDead _asbp_character_base)
        (return true)
        (else
          (Default|CallOnScreenMessage (Variables|Default|GetCaster) "Цель жива")
          (return false))))
    (:else
      (return false))))