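; Base skill that spends the owning character's stamina and mana, then heals, damages or resurrects depending on its target type.
; Healing falls back to the caster when the target isn't a character; damage hits every enemy within the area radius around an enemy target.
; Successful use starts a looping-timer cooldown, calls OnUseSkill and applies configured buffs to matching friends or enemies in that radius through the character.
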(event Custom|Use%20Skill
  (params (Target :type Character%20Object%20Reference))
  (bind _buff (Variables|Default|GetBuff))
  (bind _character (Variables|Default|GetCharacter))
  (Variables|Default|SetCurrent%20Target Target)
  ;[1 1 1] Тратим ресурсы
  (bind _asbp_character_base (Utilities|Casting|CastToBP_CharacterBase (Variables|Default|GetCharacter)))
  (Default|UseStaminaServer _asbp_character_base (Variables|Default|GetStamina%20Coast))
  (Default|UseManaServer _asbp_character_base (Variables|Default|GetMana%20Coast))
  ;[1 1 1] Проверяем соответствует ли текущая цель, цели скила (друг\враг)
  (switch Utilities|FlowControl|Switch|SwitchonESkillTarget (Variables|Default|GetTarget)
    (:NewEnumerator0
      (Utilities|Casting|CastToBP_CharacterBase (Variables|Default|GetCurrent%20Target)
        (:then
          _)
        (:CastFailed
          ;[1 1 1] Восстанавливаем здоровье себе или напарнику
          (bind _output_get (Variables|Default|SetCurrent%20Target (Variables|Default|GetCharacter)))))
      (Class|BPIBuff|RestoreHealthSkill(Message) (Variables|Default|GetCharacter) _output_get (Variables|Default|GetDamage)))
    (:NewEnumerator1
      (Utilities|Casting|CastToBP_Enemy (Variables|Default|GetCurrent%20Target))
      ;[1 1 1] Наносим урон
      (CallFunction|ApplyDamage (Variables|Default|GetCharacter) (Variables|Default|GetCurrent%20Target) (Variables|Default|GetDamage)))
    (:NewEnumerator2
      ;[1 1 1] Запуск воскрешения
      (bind _asbp_character_base_2 (Utilities|Casting|CastToBP_CharacterBase (Variables|Default|GetCurrent%20Target)))
      (Class|BPIBuff|RespawnSkill(Message) (Variables|Default|GetCharacter) _asbp_character_base_2)))
  ;[1 1 1] Устанавливаем время кулдауна
  (Variables|Default|SetCooldown%20Time (Variables|Default|GetDefault%20Cooldown%20Time))
  ;[1 1 1] Запускаем кулдаун
  (Utilities|Time|SetTimerbyFunctionName 0 "Cooldown" (Variables|Default|GetCooldown%20Tick) true)
  (Default|CallOnUseSkill self)
  ;[1 1 1] Вешаем баффы на все цели
  (if (Math|Conversions|ToBoolean(Integer) (Utilities|Array|Length _buff))
    (for _array_element _buff
      (for _array_element_2 (Utilities|Select :Index (Variables|Default|GetTarget) :NewEnumerator0 (.Friendly (Default|LineTraceArea (.AsBP%20Character%20Base (Utilities|Casting|CastToBP_CharacterBase (Variables|Default|GetCharacter))) (Transformation|GetActorLocation (Variables|Default|GetCurrent%20Target)) (Variables|Default|GetArea%20Radius))) :NewEnumerator1 (.Enemy (Default|LineTraceArea (.AsBP%20Character%20Base (Utilities|Casting|CastToBP_CharacterBase (Variables|Default|GetCharacter))) (Transformation|GetActorLocation (Variables|Default|GetCurrent%20Target)) (Variables|Default|GetArea%20Radius))) :NewEnumerator2 (.Friendly (Default|LineTraceArea (.AsBP%20Character%20Base (Utilities|Casting|CastToBP_CharacterBase (Variables|Default|GetCharacter))) (Transformation|GetActorLocation (Variables|Default|GetCurrent%20Target)) (Variables|Default|GetArea%20Radius))))
        (Class|BPIBuff|ApplyBufftoTarget(Message) _character _array_element_2 _character _array_element))))
  (Variables|Default|SetCurrent%20Target 0) ; В конце обнуляем текущую цель
)

(fn Cooldown
  (bind _output_get (Variables|Default|SetCooldown%20Time (- (Variables|Default|GetCooldown%20Time) (Variables|Default|GetCooldown%20Tick))))
  (if (<= _output_get 0.0)
    (Variables|Default|SetCooldown%20Time 0.0)
    (Utilities|Time|ClearTimerbyFunctionName 0 "Cooldown")))

(fn ApplyDamage
  (params (Character :type Character%20Object%20Reference) (Target :type Character%20Object%20Reference) (Damage :type Float%20%28single-precision%29))
  (bind _asbp_character_base (Utilities|Casting|CastToBP_CharacterBase Character))
  ;[1 1 1] Наносим урон всем целям в радиусе
  (for _array_element (.Enemy (Default|LineTraceArea _asbp_character_base (Transformation|GetActorLocation Target) (Variables|Default|GetArea%20Radius)))
    (Default|ApplyDamageServer _asbp_character_base _array_element (Variables|Default|GetDamage) _asbp_character_base)))