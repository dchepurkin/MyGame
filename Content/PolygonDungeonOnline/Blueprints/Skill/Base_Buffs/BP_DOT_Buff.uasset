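; Damage-over-time buff that periodically deals damage and sends health, mana and stamina values to its targets.
; A looping timer runs DOT Tick from BeginPlay until End Buff clears it.
; With zero radius it affects only the buff owner; otherwise it sphere-traces around the owner, choosing the object type by whether the owner is a BP_CharacterBase.
; Area hits are affected only when a visibility line trace from the owner is unblocked.
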(event EventBeginPlay
  (|CallParentFunction)
  (Utilities|Time|SetTimerbyFunctionName 0 "DOT Tick" (Variables|Buff|GetTick%20Rate) true))

(fn ConstructionScript
  (|CallParentFunction))

(fn DOTTick
  (bind _buff_owner (Variables|Default|GetBuff%20Owner))
  (bind _returnvalue (Transformation|GetActorLocation _buff_owner))
  (if (== (Variables|Buff|GetRadius) 0.0)
    (Game|Damage|ApplyDamage (Variables|Default|GetBuff%20Owner) (Variables|Buff|GetDamage) 0 (Variables|Default|GetCaster))
    (Class|BPIBuff|DOTBuff(Message) (Variables|Default|GetBuff%20Owner) (Variables|Buff|GetHealth%20Res) (Variables|Buff|GetMana%20Res) (Variables|Buff|GetStamina%20Res))
    (else
      (bind _outhits (Collision|MultiSphereTraceForObjects _returnvalue _returnvalue (Variables|Buff|GetRadius) (Utilities|Array|MakeArray (select (.bSuccess (Utilities|Casting|CastToBP_CharacterBase (Variables|Default|GetBuff%20Owner))) "ObjectTypeQuery7" "ObjectTypeQuery8")) false 0 "None" false))
      (for _array_element _outhits
        (bind _returnvalue_2 (Collision|LineTraceByChannel (Transformation|GetActorLocation (Variables|Default|GetBuff%20Owner)) (Transformation|GetActorLocation (.hitactor _array_element)) "TraceTypeQuery1" false 0 "None"))
        (if (not _returnvalue_2)
          (Game|Damage|ApplyDamage (.hitactor _array_element) (Variables|Buff|GetDamage) 0 (Variables|Default|GetCaster))
          (Class|BPIBuff|DOTBuff(Message) (.hitactor _array_element) (Variables|Buff|GetHealth%20Res) (Variables|Buff|GetMana%20Res) (Variables|Buff|GetStamina%20Res)))))))

(fn EndBuff
  (Utilities|Time|ClearTimerbyFunctionName 0 "DOT Tick"))