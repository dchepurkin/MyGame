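; Buff Blueprint that modifies aggro gain on its owner with respect to the caster.
; On BeginPlay it runs the parent logic, then sends ApplyAgroGain to the buff owner with the gain value and Caster as the aggro character.
; EndBuff sends the matching CancelAgroGain with the same values to undo the effect.
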(event EventBeginPlay
  (|CallParentFunction)
  (Class|BPIBuff|ApplyAgroGain%(Message) (Variables|Default|GetBuff%20Owner) (Variables|Buff|GetAgro%20Gain%25) (Variables|Default|GetCaster)))

(fn ConstructionScript
  (|CallParentFunction))

(fn EndBuff
  (Class|BPIBuff|CancelAgroGain%(Message) (Variables|Default|GetBuff%20Owner) (Variables|Buff|GetAgro%20Gain%25) (Variables|Default|GetCaster)))