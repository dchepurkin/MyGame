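; BP_DamageGain_Buff is a buff that changes its owner's input and output damage gain while it is active.
; On BeginPlay it runs the parent logic, then passes both gain values to the buff owner through ApplyDamageGainMessage.
; EndBuff runs the parent logic, then passes the same values to CancelDamageGainMessage, leaving the owner to apply and revert the change.
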(event EventBeginPlay
  (|CallParentFunction)
  (Class|BPIBuff|ApplyDamageGain%(Message) (Variables|Default|GetBuff%20Owner) (Variables|Buff|GetInput%20Damage%20Gain%25) (Variables|Buff|GetOutput%20Damage%20Gain%25)))

(fn ConstructionScript
  (|CallParentFunction))

(fn EndBuff
  (|CallParentFunction)
  (Class|BPIBuff|CancelDamageGain%(Message) (Variables|Default|GetBuff%20Owner) (Variables|Buff|GetInput%20Damage%20Gain%25) (Variables|Buff|GetOutput%20Damage%20Gain%25)))