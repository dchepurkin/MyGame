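; Base buff Blueprint for skills, providing a server-authoritative countdown for timed buffs on an owner.
; On BeginPlay, only the authority copies Time into CurrentTime and starts a looping one-second timer that decrements it.
; When a tick finds CurrentTime exactly zero, it clears the timer, calls EndBuff and has BuffOwner remove the buff via RemoveBuffMessage.
; EndBuff is empty here, serving as a hook for child buffs.
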(event EventBeginPlay
  (Networking|SwitchHasAuthority
    (:Authority
      (Variables|Default|SetCurrent%20Time (Variables|Buff|GetTime))
      (Utilities|Time|SetTimerbyFunctionName 0 "Timer" 1.0 true))))

(fn ConstructionScript)

(fn Timer
  (if (== (Variables|Default|GetCurrent%20Time) 0.0)
    (Utilities|Time|ClearTimerbyFunctionName 0 "Timer")
    (CallFunction|EndBuff)
    (Class|BPIBuff|RemoveBuff(Message) (Variables|Default|GetBuff%20Owner) self)
    (else
      (bind _result (Math|Float|DecrementFloat (Variables|Default|GetCurrent%20Time))
        (:%20%20
          (Variables|Default|SetCurrent%20Time _result))))))

(fn EndBuff)