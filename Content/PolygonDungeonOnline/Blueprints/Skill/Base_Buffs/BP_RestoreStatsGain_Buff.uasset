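; Buff Blueprint that temporarily changes its owner's health, mana and stamina restore gains.
; On BeginPlay it calls the parent logic, then sends the three gain values to BuffOwner through ApplyRestoreStatsGain.
; EndBuff calls the parent logic, then passes the same values to CancelRestoreStatsGain to reverse the effect.
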(event EventBeginPlay
  (|CallParentFunction)
  (Class|BPIBuff|ApplyRestoreStatsGain%(Message) (Variables|Default|GetBuff%20Owner) (Variables|Buff|GetHealth%20Res%20Gain%25) (Variables|Buff|GetMana%20Res%20Gain%25) (Variables|Buff|GetStamina%20Res%20Gain%25)))

(fn ConstructionScript
  (|CallParentFunction))

(fn EndBuff
  (|CallParentFunction)
  (Class|BPIBuff|CancelRestoreStatsGain%(Message) (Variables|Default|GetBuff%20Owner) (Variables|Buff|GetHealth%20Res%20Gain%25) (Variables|Buff|GetMana%20Res%20Gain%25) (Variables|Buff|GetStamina%20Res%20Gain%25)))