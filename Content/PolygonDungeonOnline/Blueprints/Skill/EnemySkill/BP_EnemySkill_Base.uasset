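; BP_EnemySkill_Base is a base Blueprint for enemy skills that deal damage and apply buffs to targets.
; UseSkill stores the passed targets and caster, then damages each target only when the skill's Target type is enemy-targeted.
; It then sends every configured buff to every target through ApplyBuffMessage with the caster, regardless of target type.
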(event Custom|Use%20Skill
  (params (Skill%20Target :type Array%20of%20Character%20Object%20References) (Caster :type Character%20Object%20Reference))
  (Variables|Default|SetCurrent%20Targets Skill%20Target)
  (Variables|Default|SetCaster Caster)
  (Utilities|FlowControl|Sequence
    (:then_0
      (switch Utilities|FlowControl|Switch|SwitchonESkillTarget (Variables|Default|GetTarget)
        (:NewEnumerator1
          ;[1 1 1] Наносим урон целям
          (for _array_element (Variables|Default|GetCurrent%20Targets)
            (Game|Damage|ApplyDamage _array_element (Variables|Default|GetDamage) 0 0)))))
    (:then_1
      ;[1 1 1] Вешаем бафы
      (if (Math|Conversions|ToBoolean(Integer) (Utilities|Array|Length (Variables|Default|GetBuffs)))
        (for _array_element_2 (Variables|Default|GetBuffs)
          (for _array_element_3 (Variables|Default|GetCurrent%20Targets)
            (Class|BPIBuff|ApplyBuff(Message) _array_element_3 (Variables|Default|GetCaster) _array_element_2)))))))