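; BP_Respawn_Skill is a resurrection skill that revives a dead BP_CharacterBase target.
; SetTarget accepts only that character class, with Russian on-screen errors for enemy or missing targets.
; IsTargetAvailable checks distance and validity and requires the target to be dead.
; EndSkill sends the caster a respawn message for the target, then CastBuffs has the caster apply each of the skill's buffs to it.
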(event EventBeginPlay)

(event Collision|EventActorBeginOverlap
  (params (OtherActor :type Actor%20Object%20Reference)))

(event EventTick
  (params (DeltaSeconds :type Float%20%28single-precision%29)))

(fn ConstructionScript
  (|CallParentFunction))

(fn SetTarget
  (params (Cast%20Target :type Character%20Object%20Reference))
  (bind _caster (Variables|Default|GetCaster))
  (bind _asbp_character_base (Utilities|Casting|CastToBP_CharacterBase Cast%20Target)
    (:then
      (Variables|Default|SetCast%20Target _asbp_character_base)
      (return true))
    (:CastFailed
      (Utilities|Casting|CastToBP_Enemy Cast%20Target
        (:then
          (Default|CallOnScreenMessage _caster "Неподходящая цель"))
        (:CastFailed
          (Default|CallOnScreenMessage _caster "Нет цели")))
      (return false))))

(fn IsTargetAvailable
  (if (CallFunction|CheckDistanse)
    (bind _cast_target (Variables|Default|GetCast%20Target)
      (:then
        (bind _asbp_character_base (Utilities|Casting|CastToBP_CharacterBase _cast_target))
        (if (Variables|/Game/PolygonDungeonOnline/Character/Blueprints/BP_CharacterBase.BP_CharacterBase_C|GetIsDead _asbp_character_base)
          (return true)
          (else
            (Default|CallOnScreenMessage (Variables|Default|GetCaster) "Цель жива")
            (return false))))
      (:else
        (return false)))))

(fn EndSkill
  (bind _asbp_character_base (Utilities|Casting|CastToBP_CharacterBase (Variables|Default|GetCast%20Target)))
  (Class|BPIBuff|RespawnSkill(Message) (Variables|Default|GetCaster) _asbp_character_base)
  (CallFunction|CastBuffs))

(fn CastBuffs
  (bind _caster (Variables|Default|GetCaster))
  (for _array_element (Variables|Default|GetBuffs)
    (Class|BPIBuff|ApplyBufftoTarget(Message) _caster (Variables|Default|GetCast%20Target) _caster _array_element)))