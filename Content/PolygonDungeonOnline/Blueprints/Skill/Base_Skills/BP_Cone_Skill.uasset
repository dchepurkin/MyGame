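; Cone-shaped area skill that heals friendly or damages enemy characters in front of player character 0, depending on its target type.
; On skill end, it fans multi-object line traces at one-degree steps from just above the capsule's base, with debug drawing on.
; Unique blocking-hit characters visible to the caster become targets, then receive healing or damage plus each configured buff through caster calls.
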(fn ConstructionScript
  (|CallParentFunction))

(fn SetTarget
  (params (Cast%20Target :type Character%20Object%20Reference))
  (Variables|Default|SetCast%20Target Cast%20Target)
  (return true))

(fn IsTargetAvailable
  (return true))

(fn EndSkill
  (CallFunction|LineTraceforArea)
  (CallFunction|ApplyDamage)
  (CallFunction|ApplyBuffs))

(fn GetStartPoint
  (params (Character :type Character%20Object%20Reference))
  (bind _returnvalue (Transformation|GetActorLocation Character))
  (bind (_x _y _z) (Math|Vector|BreakVector _returnvalue))
  (bind _capsulecomponent (Variables|/Script/Engine.Character|GetCapsuleComponent Character)
    (:then
      (return (Math|Vector|MakeVector _x _y (+ (- _z (Variables|/Script/Engine.CapsuleComponent|GetCapsuleHalfHeight _capsulecomponent)) 5.0))))
    (:else
      (return "0, 0, 0"))))

(fn LineTraceforArea
  (bind _returnvalue (Game|GetPlayerCharacter 0))
  (bind _start_point (CallFunction|GetStartPoint _returnvalue))
  (Utilities|Array|Clear (Variables|Default|GetTargets))
  (for _index (range 0 (Math|Float|Truncate (* (Variables|Default|GetHalf%20Ange) 2.0)))
    (bind _outhits (Class|KismetSystemLibrary|LineTraceMultiforObjects _start_point (+ _start_point (* (Math|Vector|RotateVectorAroundAxis (Transformation|GetActorForwardVector _returnvalue) (+ (Math|Conversions|ToFloat(Integer) _index) (* (Variables|Default|GetHalf%20Ange) -1.0)) "0, 0,1.000000") (Variables|Default|GetSkill%20Radius))) (Utilities|Array|MakeArray (Utilities|Select :Index (Variables|Default|GetTarget) :NewEnumerator0 "ObjectTypeQuery7" :NewEnumerator1 "ObjectTypeQuery8")) false (Utilities|Array|MakeArray (Variables|Default|GetCaster)) "ForDuration" true))
    (for _array_element _outhits
      (if (.bblockinghit _array_element)
        (bind _ascharacter (Utilities|Casting|CastToCharacter (.hitactor _array_element)))
        (if (Default|GetTargetVisibleonCharacter (Variables|Default|GetCaster) _ascharacter)
          (Utilities|Array|AddUnique (Variables|Default|GetTargets) _ascharacter))))))

(fn ApplyBuffs
  (bind _caster (Variables|Default|GetCaster))
  (for _array_element (Variables|Default|GetTargets)
    (for _array_element_2 (Variables|Default|GetBuff)
      (Class|BPIBuff|ApplyBufftoTarget(Message) _caster _array_element _caster _array_element_2))))

(fn ApplyDamage
  (bind _caster (Variables|Default|GetCaster))
  (switch Utilities|FlowControl|Switch|SwitchonESkillTarget (Variables|Default|GetTarget)
    (:NewEnumerator0
      (for _array_element (Variables|Default|GetTargets)
        (Default|RestoreHealthSkill (Variables|Default|GetCaster) _array_element (Variables|Default|GetDamage))))
    (:NewEnumerator1
      (for _array_element_2 (Variables|Default|GetTargets)
        (Default|ApplyDamageServer _caster _array_element_2 (Variables|Default|GetDamage) _caster))))
  (return true))