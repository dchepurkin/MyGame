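; BP_StatSphere_Skill is a skill that spends a share of the caster's health, mana or stamina to spawn a sphere of that stat type.
; CanUse blocks casting with a Russian on-screen message unless the current stat exceeds the StatNeed fraction of its maximum.
; StartSkill calls ApplySkill without needing a target.
; EndSkill deducts the cost through server calls, using self-damage for health, then spawns the sphere with StatRestore.
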(fn ConstructionScript
  (|CallParentFunction))

(fn IsTargetAvailable
  (return true))

(fn CanUse
  (bind _caster (Variables|Default|GetCaster))
  (bind _caster_2 (Variables|Default|GetCaster))
  (if (>= (* (Utilities|Select :Index (Variables|Skill|GetStat) :NewEnumerator0 (Variables|/Game/PolygonDungeonOnline/Character/Blueprints/BP_CharacterBase.BP_CharacterBase_C|GetMax%20Health _caster) :NewEnumerator1 (Variables|/Game/PolygonDungeonOnline/Character/Blueprints/BP_CharacterBase.BP_CharacterBase_C|GetMax%20Mana _caster) :NewEnumerator2 (Variables|/Game/PolygonDungeonOnline/Character/Blueprints/BP_CharacterBase.BP_CharacterBase_C|GetMax%20Stamina _caster)) (Variables|Skill|GetStatNeed%25)) (Utilities|Select :Index (Variables|Skill|GetStat) :NewEnumerator0 (Variables|/Game/PolygonDungeonOnline/Character/Blueprints/BP_CharacterBase.BP_CharacterBase_C|GetCurrent%20Health _caster_2) :NewEnumerator1 (Variables|/Game/PolygonDungeonOnline/Character/Blueprints/BP_CharacterBase.BP_CharacterBase_C|GetCurrent%20Mana _caster_2) :NewEnumerator2 (Variables|/Game/PolygonDungeonOnline/Character/Blueprints/BP_CharacterBase.BP_CharacterBase_C|GetCurrent%20Stamina _caster_2)))
    (Default|CallOnScreenMessage (Variables|Default|GetCaster) (Utilities|Text|FormatText "Не хватает {S}" (Utilities|Select :Index (Variables|Skill|GetStat) :NewEnumerator0 "здоровья" :NewEnumerator1 "маны" :NewEnumerator2 "запаса сил")))
    (return false)
    (else
      (return (|CallParentFunction)))))

(fn StartSkill
  (CallFunction|ApplySkill))

(fn EndSkill
  (bind _caster (Variables|Default|GetCaster))
  (bind _caster_2 (Variables|Default|GetCaster))
  (bind _caster_3 (Variables|Default|GetCaster))
  (Utilities|FlowControl|Sequence
    (:then_0
      (switch Utilities|FlowControl|Switch|SwitchonE_Stat (Variables|Skill|GetStat)
        (:NewEnumerator0
          (Default|ApplyDamageServer _caster_2 _caster_2 (* (Variables|/Game/PolygonDungeonOnline/Character/Blueprints/BP_CharacterBase.BP_CharacterBase_C|GetMax%20Health _caster_2) (Variables|Skill|GetStatNeed%25)) _caster_2))
        (:NewEnumerator1
          (Default|UseManaServer _caster_3 (* (Variables|/Game/PolygonDungeonOnline/Character/Blueprints/BP_CharacterBase.BP_CharacterBase_C|GetMax%20Mana _caster_3) (Variables|Skill|GetStatNeed%25))))
        (:NewEnumerator2
          (Default|UseStaminaServer _caster (* (Variables|/Game/PolygonDungeonOnline/Character/Blueprints/BP_CharacterBase.BP_CharacterBase_C|GetMax%20Stamina _caster) (Variables|Skill|GetStatNeed%25))))))
    (:then_1
      (Default|SpawnStatSphere (Variables|Default|GetCaster) (Variables|Skill|GetStat) (Variables|Skill|GetStatRestore%25)))))

(fn SetTarget
  (params (Cast%20Target :type Character%20Object%20Reference))
  (return true))