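; Base skill for ground-placed area-of-effect abilities that need no target validation, as both target checks always pass.
; Initialize spawns a BP_AOE_Area owned by player 0, passing it the radius, max distance and skill reference.
; Cast AOE stores the location and has the caster play the montage via the server, while Cancel clears the caster's current skill.
; End Skill has the caster spawn the AOE there with damage, timing and buffs.
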(fn ConstructionScript
  (|CallParentFunction))

(fn SetTarget
  (params (Cast%20Target :type Character%20Object%20Reference))
  (return true))

(fn IsTargetAvailable
  (return true))

(fn Initialize
  (Game|SpawnActorfromClass "/Game/PolygonDungeonOnline/Blueprints/Skill/BP_AOE_Area.BP_AOE_Area_C" (Math|Transform|MakeTransform "0, 0, 0" "0, 0, 0" "1,1,1") "AlwaysSpawn" (Game|GetPlayerCharacter 0) (Variables|Default|GetSkill%20Radius) (Variables|Default|GetMax%20Distance) self 0))

(fn CastAOE
  (params (AOE%20Location :type Vector))
  (Variables|Default|SetAOE%20Location AOE%20Location)
  (Default|PlaySkillMontageServer (Variables|Default|GetCaster) (Variables|Default|GetAnimMontage)))

(fn CancelAOE
  (Variables|/Game/PolygonDungeonOnline/Character/Blueprints/BP_CharacterBase.BP_CharacterBase_C|SetCurrent%20Skill (Variables|Default|GetCaster) 0))

(fn EndSkill
  (|CallParentFunction)
  (Default|SpawnAOE (Variables|Default|GetCaster) (Math|Transform|MakeTransform (Variables|Default|GetAOE%20Location) "0, 0, 0" "1,1,1") (Variables|Default|GetSkill%20Radius) (Variables|Default|GetDamage) (Variables|Default|GetTime) (Variables|Default|GetAOE%20Tick%20Rate) (Variables|Default|GetCaster) (Variables|Default|GetBuff) (Variables|Default|GetTarget)))