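; BP_RangeTargetSkill is a base skill Blueprint for ranged skills that launch a projectile at a cast target.
; BeginPlay sets the targeting rules: ignore the caster, not self-only, and a preset target type.
; When the skill ends, it asks the caster to spawn the projectile from a named mesh socket, passing along damage, radii, initial speed, target and buffs.
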(event EventBeginPlay
  (Variables|Default|SetIgnore%20Self true)
  (Variables|Default|SetSelf%20Only false)
  (Variables|Default|SetTarget "NewEnumerator1"))

(fn ConstructionScript
  (|CallParentFunction))

(fn EndSkill
  (Default|SpawnRangeProjectile (Variables|Default|GetCaster) (Variables|Skill|GetProjectile) (Transformation|GetSocketTransform (Variables|/Script/Engine.Character|GetMesh (Variables|Default|GetCaster)) (Variables|Default|GetSocket%20Name) "RTS_World") (Variables|Default|GetDamage) (Variables|Default|GetDamage%20Radius) (Variables|Default|GetBuff%20Radius) (Variables|Skill|GetInit%20Speed) (Variables|Default|GetCast%20Target) (Variables|Default|GetBuffs)))