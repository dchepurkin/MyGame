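; Base Blueprint for character skills, handling use checks, targeting, resource costs and cooldown.
; UseSkill gates on caster state, montages, cooldown, stamina and mana, then validates target range and visibility before StartSkill plays the montage through a server call.
; A separate ApplySkill event spends resources, runs a looping cooldown timer, broadcasts use and calls EndSkill.
; SetTarget (false by default) and empty EndSkill act as child hooks.
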(event Custom|Apply%20Skill
  (bind _caster (Variables|Default|GetCaster))
  (Default|UseStaminaServer _caster (Variables|Skill|GetStamina%20Coast))
  (Default|UseManaServer _caster (Variables|Skill|GetMana%20Coast))
  (Variables|Default|SetCurrent%20Cooldown%20Time (Variables|Skill|GetCooldown%20Time))
  (Utilities|Time|SetTimerbyFunctionName 0 "Cooldown" (Variables|Default|GetCooldown%20Tick) true)
  (Default|CallOnUseSkill self)
  (CallFunction|EndSkill)
  (Variables|Default|SetCast%20Target 0) ; В конце обнуляем текущую цель
)

(event Custom|Use%20Skill
  (params (Cast%20Target :type Character%20Object%20Reference))
  (if (CallFunction|CanUse)
    (Variables|Default|SetCast%20Target 0)
    (bind _success (CallFunction|SetTarget Cast%20Target))
    (if _success
      (if (CallFunction|IsTargetAvailable)
        (Variables|/Game/PolygonDungeonOnline/Character/Blueprints/BP_CharacterBase.BP_CharacterBase_C|SetCurrent%20Skill (Variables|Default|GetCaster) self)
        (CallFunction|StartSkill)))))

(fn ConstructionScript)

(fn CanUse
  (bind _caster (Variables|Default|GetCaster))
  (bind _caster_2 (Variables|Default|GetCaster))
  (bind _caster_3 (Variables|Default|GetCaster))
  (Variables|/Game/PolygonDungeonOnline/Character/Blueprints/BP_CharacterBase.BP_CharacterBase_C|GetCurrent%20Skill (Variables|Default|GetCaster)
    (:then
      (return false))
    (:else
      (if (Math|Boolean|ANDBoolean (Utilities|Enum|NotEqual(Enum) (Variables|/Game/PolygonDungeonOnline/Character/Blueprints/BP_CharacterBase.BP_CharacterBase_C|GetPose _caster) "NewEnumerator0") (not (Variables|/Game/PolygonDungeonOnline/Character/Blueprints/BP_CharacterBase.BP_CharacterBase_C|GetIsDead _caster)) (not (Variables|/Game/PolygonDungeonOnline/Character/Blueprints/BP_CharacterBase.BP_CharacterBase_C|GetIsBlock _caster)) (not (Default|IsJumping _caster)) (not (Variables|/Game/PolygonDungeonOnline/Character/Blueprints/BP_CharacterBase.BP_CharacterBase_C|GetStun _caster)))
        (bind _values (Utilities|Map|Values (Variables|/Game/PolygonDungeonOnline/Character/Blueprints/BP_CharacterBase.BP_CharacterBase_C|GetEnableWeaponMontages _caster_2)))
        (if (not (Utilities|Array|ContainsItem _values (.Montage (Default|GetMontagePlaying _caster_2)))) ; во время экипировки оружия нельзя юзать скилл
          (bind _values_2 (Utilities|Map|Values (Variables|/Game/PolygonDungeonOnline/Character/Blueprints/BP_CharacterBase.BP_CharacterBase_C|GetRoll%20Montages _caster_3)))
          (if (not (Utilities|Array|ContainsItem _values_2 (.Montage (Default|GetMontagePlaying _caster_3)))) ; Если воспроизводится перекат то скил юзать нельзя
            (if (== (Variables|Default|GetCurrent%20Cooldown%20Time) 0.0)
              (if (>= (Variables|/Game/PolygonDungeonOnline/Character/Blueprints/BP_CharacterBase.BP_CharacterBase_C|GetCurrent%20Stamina (Variables|Default|GetCaster)) (Variables|Skill|GetStamina%20Coast))
                (if (>= (Variables|/Game/PolygonDungeonOnline/Character/Blueprints/BP_CharacterBase.BP_CharacterBase_C|GetCurrent%20Mana (Variables|Default|GetCaster)) (Variables|Skill|GetMana%20Coast))
                  (return true)
                  (else
                    (Default|CallOnScreenMessage (Variables|Default|GetCaster) "Не хватает маны")))
                (else
                  (Default|CallOnScreenMessage (Variables|Default|GetCaster) "Не хватает запаса сил")))
              (return false)
              (else
                _)))
          (return false)
          (else
            (return false)))
        (else
          (return false))))))

(fn SetTarget
  (params (Cast%20Target :type Character%20Object%20Reference))
  (return false))

(fn IsTargetAvailable
  (return (CallFunction|CheckDistanse)))

(fn CheckDistanse
  (bind _cast_target (Variables|Default|GetCast%20Target)
    (:then
      (if (<= (Transformation|GetDistanceTo (Variables|Default|GetCaster) _cast_target) (Variables|Skill|GetMin%20Distance))
        (if (Default|GetTargetVisibleonCharacter (Variables|Default|GetCaster) (Variables|Default|GetCast%20Target))
          (return true)
          (else
            (Default|CallOnScreenMessage (Variables|Default|GetCaster) "Цель не видна")
            (return false)))
        (else
          (Default|CallOnScreenMessage (Variables|Default|GetCaster) "Цель слишком далеко")
          (return false))))
    (:else
      (Default|CallOnScreenMessage (Variables|Default|GetCaster) "Нет цели")
      (return false))))

(fn StartSkill
  (Default|PlaySkillMontageServer (Variables|Default|GetCaster) (Variables|Skill|GetAnimation)))

(fn Cooldown
  (bind _output_get (Variables|Default|SetCurrent%20Cooldown%20Time (- (Variables|Default|GetCurrent%20Cooldown%20Time) (Variables|Default|GetCooldown%20Tick))))
  (if (<= _output_get 0.0)
    (Variables|Default|SetCurrent%20Cooldown%20Time 0.0)
    (Utilities|Time|ClearTimerbyFunctionName 0 "Cooldown")))

(fn EndSkill)