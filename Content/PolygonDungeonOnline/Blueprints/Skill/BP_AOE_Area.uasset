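; Targeting indicator actor for area-of-effect skills, letting the player pick a cast point with the mouse.
; Each tick it follows the cursor trace, capped at the character's foot height, and tints cyan within MaxDistance or red beyond.
; A looping timer spins the Area component, which is scaled from Radius.
; Left click in range calls CastAOE on Skill, Escape calls CancelAOE, and either destroys the actor.
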(event EventBeginPlay
  (bind _returnvalue (Game|GetPlayerController 0))
  (bind _radius (Variables|Default|GetRadius))
  (bind _returnvalue_2 (/ _radius 5e+01))
  (bind (_sizex _sizey) (HUD|GetViewportSize _returnvalue))
  (Class|PlayerController|SetMouseLocation _returnvalue (/ _sizex 2) (/ _sizey 2))
  (Transformation|SetRelativeScale3D (Variables|Default|GetArea) (Math|Vector|MakeVector _returnvalue_2 0.0 _returnvalue_2))
  (Utilities|Time|SetTimerbyFunctionName 0 "SetRotation" 0.01 true))

(event EventTick
  (params (DeltaSeconds :type Float%20%28single-precision%29))
  (bind _returnvalue (Game|GetPlayerController 0))
  (bind _hitresult (Game|Player|GetHitResultUnderCursorbyChannel _returnvalue "TraceTypeQuery2" true))
  (Transformation|SetActorLocation (CallFunction|GetLocation (.impactpoint _hitresult)) false false)
  (Rendering|Material|SetVectorParameterValueonMaterials (Variables|Default|GetArea) "Color" (Math|Conversions|ToVector(LinearColor) (Math|Color|SelectColor "(R=0.294118,G=0.968628,B=1.000000,A=1.000000)" "(R=1.000000,G=0.000000,B=0.014804,A=1.000000)" (< (Math|Vector|Distance(Vector) (.impactpoint _hitresult) (Transformation|GetActorLocation (Game|GetPlayerCharacter 0))) (Variables|Default|GetMax%20Distance))))))

(event Input|MouseEvents|LeftMouseButton
  (params (Key :type Key%20Structure))
  (bind _returnvalue (Game|GetPlayerController 0))
  (bind _hitresult (Game|Player|GetHitResultUnderCursorbyChannel _returnvalue "TraceTypeQuery2" true))
  (:Pressed
    (if (< (Math|Vector|Distance(Vector) (.impactpoint _hitresult) (Transformation|GetActorLocation (Game|GetPlayerCharacter 0))) (Variables|Default|GetMax%20Distance))
      (Default|CastAOE (Variables|Default|GetSkill) (.impactpoint _hitresult))
      (Actor|DestroyActor))))

(event Input|KeyboardEvents|Escape
  (params (Key :type Key%20Structure))
  (:Pressed
    (Default|CancelAOE (Variables|Default|GetSkill))
    (Actor|DestroyActor)))

(fn ConstructionScript)

(fn SetRotation
  (Transformation|AddRelativeRotation (Variables|Default|GetArea) "0,0.250000, 0" true false))

(fn GetLocation
  (params (Trace%20Location :type Vector))
  (bind (_x _y _z) (Math|Vector|BreakVector Trace%20Location))
  (bind _returnvalue (Game|GetPlayerCharacter 0))
  (bind _returnvalue_2 (Transformation|GetActorLocation _returnvalue))
  (bind _capsulecomponent (Variables|/Script/Engine.Character|GetCapsuleComponent _returnvalue))
  (bind _returnvalue_3 (Components|Capsule|GetScaledCapsuleHalfHeight _capsulecomponent))
  (bind _returnvalue_4 (- (.z _returnvalue_2) _returnvalue_3))
  (if (> _z _returnvalue_4)
    (return (Math|Vector|MakeVector _x _y _returnvalue_4))
    (else
      (return Trace%20Location))))