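; BP_AOE is a timed area-of-effect skill zone that either heals friendly characters or damages hostile targets, applying buffs in both modes.
; The server runs a looping Make Damage timer until the lifespan ends, while clients scale and tint the area mesh by target type.
; Friendly ticks heal overlapping characters; hostile ticks deal caster-scaled radial damage ignoring all BP_CharacterBase actors, then buff overlapping BP_Enemy actors.
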(event EventBeginPlay
  (bind _radius (Variables|Default|GetRadius))
  (bind _sm_aoe_skill (Variables|Default|GetSM_AOE_Skill))
  (bind _returnvalue (/ _radius 5e+01))
  (Components|Sphere|SetSphereRadius (Variables|Default|GetAOE) _radius true)
  (Networking|SwitchHasAuthority
    (:Authority
      (Utilities|Time|SetTimerbyFunctionName 0 "Make Damage" (Variables|Default|GetTick%20Rate) true)
      (Actor|SetLifeSpan (Variables|Default|GetTime)))
    (:Remote
      (Transformation|SetRelativeScale3D _sm_aoe_skill (Math|Vector|MakeVector _returnvalue _returnvalue 0.0))
      (Rendering|Material|SetVectorParameterValueonMaterials _sm_aoe_skill "Color" (Math|Conversions|ToVector(LinearColor) (Utilities|Select :Index (Variables|Default|GetTarget) :NewEnumerator0 "(R=0.000000,G=1.000000,B=0.000000,A=0.047059)" :NewEnumerator1 "(R=0.000000,G=0.000000,B=1.000000,A=0.050000)"))))))

(event EventDestroyed
  (Utilities|Time|ClearTimerbyFunctionName 0 "Make Damage"))

(fn ConstructionScript)

(fn MakeDamage
  (bind _caster (Variables|Default|GetCaster))
  (bind _asbp_character_base (Utilities|Casting|CastToBP_CharacterBase _caster))
  (Networking|SwitchHasAuthority
    (:Authority
      (switch Utilities|FlowControl|Switch|SwitchonESkillTarget (Variables|Default|GetTarget)
        (:NewEnumerator0
          (for _array_element (Collision|GetOverlappingActors (Variables|Default|GetAOE) "/Game/PolygonDungeonOnline/Character/Blueprints/BP_CharacterBase.BP_CharacterBase_C" :!class /Script/Engine.PrimitiveComponent)
            (bind _asbp_character_base_2 (Utilities|Casting|CastToBP_CharacterBase _array_element))
            (Default|RestoreHealthServer _asbp_character_base_2 (Variables|Default|GetDamage))
            (for _array_element_2 (Variables|Default|GetBuffs)
              (Default|ApplyBuff _asbp_character_base_2 (Variables|Default|GetCaster) _array_element_2))))
        (:NewEnumerator1
          (bind _outactors (Actor|GetAllActorsOfClass "/Game/PolygonDungeonOnline/Character/Blueprints/BP_CharacterBase.BP_CharacterBase_C"))
          (Game|Damage|ApplyRadialDamage (* (Variables|Default|GetDamage) (Variables|/Game/PolygonDungeonOnline/Character/Blueprints/BP_CharacterBase.BP_CharacterBase_C|GetOutput%20Damage%20Gain%25 _asbp_character_base)) (Transformation|GetActorLocation) (Variables|Default|GetRadius) 0 _outactors _asbp_character_base 0 true "ECC_Visibility")
          (for _array_element_3 (Collision|GetOverlappingActors (Variables|Default|GetAOE) "/Game/PolygonDungeonOnline/Enemy/Blueprints/BP_Enemy.BP_Enemy_C" :!class /Script/Engine.PrimitiveComponent)
            (bind _asbp_enemy (Utilities|Casting|CastToBP_Enemy _array_element_3))
            (for _array_element_4 (Variables|Default|GetBuffs)
              (Default|ApplyBuff _asbp_enemy (Variables|Default|GetCaster) _array_element_4))))))))