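; Base buff actor that applies a timed effect from a caster to its owner, with the kind chosen by BuffType.
; On BeginPlay the server applies it through messages to the owner: shield, damage over time, aggro gain or target lock, restore gain, damage modifiers, slowdown or stun.
; A looping timer counts down the duration, then reverses the effect and asks the owner to remove the buff.
; DOT buffs tick separately, dealing damage and sending resource-restore amounts.
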(event EventBeginPlay
  (Networking|SwitchHasAuthority
    (:Authority
      (Variables|Default|SetCurrent%20Time (Variables|Default|GetTime))
      (Utilities|Time|SetTimerbyFunctionName 0 "Set Current Time" 1.0 true)
      (switch Utilities|FlowControl|Switch|SwitchonEBuffType (Variables|Default|GetBuff%20Type)
        (:NewEnumerator0
          (Class|BPIBuff|ApplyShieldPowerGain%(Message) (Variables|Default|GetBuff%20Owner) (Variables|Gain|GetShield%20Power%20Gain%25)))
        (:NewEnumerator1
          (Utilities|Time|SetTimerbyFunctionName 0 "DOT Damage" (Variables|DOT|GetDOT%20Tick) true))
        (:NewEnumerator2
          (Class|BPIBuff|ApplyAgroGain%(Message) (Variables|Default|GetBuff%20Owner) (Variables|Gain|GetAgro%20Gain%25) (Variables|Default|GetCaster)))
        (:NewEnumerator5
          (Class|BPIBuff|ApplyAgroTarget(Message) (Variables|Default|GetBuff%20Owner) false (Variables|Default|GetCaster)))
        (:NewEnumerator3
          (Class|BPIBuff|ApplyRestoreStatsGain%(Message) (Variables|Default|GetBuff%20Owner) (Variables|Gain|GetHealth%20Res%20Gain%25) (Variables|Gain|GetMana%20Res%20Gain%25) (Variables|Gain|GetStamina%20Res%20Gain%25)))
        (:NewEnumerator4
          (Class|BPIBuff|ApplyDamageGain%(Message) (Variables|Default|GetBuff%20Owner) (Variables|Gain|GetInput%20Damage%20Gain%25) (Variables|Gain|GetOutput%20Damage%20Gain%25)))
        (:NewEnumerator6
          (Class|BPIBuff|ApplySlowdown%(Message) (Variables|Default|GetBuff%20Owner) (Variables|Movement|GetSlowdown%25)))
        (:NewEnumerator7
          (Class|BPIBuff|ApplyStan(Message) (Variables|Default|GetBuff%20Owner) true))))))

(fn ConstructionScript)

(fn SetCurrentTime
  (if (== (Variables|Default|GetCurrent%20Time) 0.0)
    (Utilities|Time|ClearTimerbyFunctionName 0 "Set Current Time")
    (Utilities|FlowControl|Sequence
      (:then_0
        (switch Utilities|FlowControl|Switch|SwitchonEBuffType (Variables|Default|GetBuff%20Type)
          (:NewEnumerator0
            (Class|BPIBuff|CancelShieldPowerGain%(Message) (Variables|Default|GetBuff%20Owner) (Variables|Gain|GetShield%20Power%20Gain%25)))
          (:NewEnumerator1
            (Utilities|Time|ClearTimerbyFunctionName 0 "DOT Damage"))
          (:NewEnumerator2
            (Class|BPIBuff|CancelAgroGain%(Message) (Variables|Default|GetBuff%20Owner) (Variables|Gain|GetAgro%20Gain%25) (Variables|Default|GetCaster)))
          (:NewEnumerator5
            (Class|BPIBuff|ApplyAgroTarget(Message) (Variables|Default|GetBuff%20Owner) true (Variables|Default|GetCaster)))
          (:NewEnumerator3
            (Class|BPIBuff|CancelRestoreStatsGain%(Message) (Variables|Default|GetBuff%20Owner) (Variables|Gain|GetHealth%20Res%20Gain%25) (Variables|Gain|GetMana%20Res%20Gain%25) (Variables|Gain|GetStamina%20Res%20Gain%25)))
          (:NewEnumerator4
            (Class|BPIBuff|CancelDamageGain%(Message) (Variables|Default|GetBuff%20Owner) (Variables|Gain|GetInput%20Damage%20Gain%25) (Variables|Gain|GetOutput%20Damage%20Gain%25)))
          (:NewEnumerator6
            (Class|BPIBuff|CancelSlowdown%(Message) (Variables|Default|GetBuff%20Owner) (Variables|Movement|GetSlowdown%25)))
          (:NewEnumerator7
            (Class|BPIBuff|ApplyStan(Message) (Variables|Default|GetBuff%20Owner) false))))
      (:then_1
        (Class|BPIBuff|RemoveBuff(Message) (Variables|Default|GetBuff%20Owner) self)))
    (else
      (bind _result (Math|Float|DecrementFloat (Variables|Default|GetCurrent%20Time))
        (:%20%20
          (Variables|Default|SetCurrent%20Time _result))))))

(fn DOTDamage
  (Game|Damage|ApplyDamage (Variables|Default|GetBuff%20Owner) (Variables|DOT|GetDamage%20DOT) 0 (Variables|Default|GetCaster))
  (Class|BPIBuff|DOTBuff(Message) (Variables|Default|GetBuff%20Owner) (Variables|DOT|GetHealth%20Res%20Dot) (Variables|DOT|GetMana%20Res%20Dot) (Variables|DOT|GetStamina%20Res%20Dot)))