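; BP_Tank is a tank character Blueprint that adds outline-style target highlighting to its modular body and gear meshes.
; InTarget casts the target to BP_Tank, enables custom depth on its meshes and sets their stencil value by whether it is the CurrentTarget.
; OffTarget disables custom depth on the same meshes.
; The event graph is empty, and the construction script only calls its parent.
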(event EventBeginPlay)

(event Collision|EventActorBeginOverlap
  (params (OtherActor :type Actor%20Object%20Reference)))

(event EventTick
  (params (DeltaSeconds :type Float%20%28single-precision%29)))

(fn ConstructionScript
  (|CallParentFunction))

(fn InTarget
  (params (Target :type Character%20Object%20Reference))
  (bind _asbp_tank (Utilities|Casting|CastToBP_Tank Target))
  (Rendering|SetCustomDepthStencilValue (Variables|BP_Tank_C|GetHelm _asbp_tank) (Math|Integer|SelectInt 1 0 (== (Variables|Default|GetCurrent%20Target) Target)))
  (Rendering|SetRenderCustomDepth (Variables|/Script/Engine.Character|GetMesh _asbp_tank) true))

(fn OffTarget
  (params (Target :type Character%20Object%20Reference))
  (bind _asbp_tank (Utilities|Casting|CastToBP_Tank Target))
  (Rendering|SetRenderCustomDepth (Variables|/Script/Engine.Character|GetMesh _asbp_tank) false))