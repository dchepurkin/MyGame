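; Player controller for an online game that spawns and possesses the player's chosen character.
; On BeginPlay it sets game-only input, and only the non-authority side passes the class and name from BP_GameInstance to SpawnCharacterServer.
; That event spawns the pawn at the first PlayerStart found and possesses it.
; Possession turns on the FPS stat, and unpossession notifies the game instance for a server player-count check.
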(event Custom|Spawn%20Character%20Server
  (params (Character :type BP%20Character%20Base%20Class%20Reference) (Character%20Name :type Name))
  ;[1 1 1] Спавним Персонажа
  (bind _returnvalue (Actor|GetActorOfClass "/Script/Engine.PlayerStart"))
  (if (Utilities|IsValidClass Character)
    (bind _returnvalue_2 (Game|SpawnActorfromClass Character (Math|Transform|MakeTransform (Transformation|GetActorLocation _returnvalue) "0, 0, 0" "1,1,1") "AlwaysSpawn" 0 Character%20Name 0))
    (Pawn|Possess _returnvalue_2)))

(event EventPossess
  (params (PossessedPawn :type Pawn%20Object%20Reference))
  (Development|ExecuteConsoleCommand "stat FPS" 0))

(event EventUnPossess
  (params (UnpossessedPawn :type Pawn%20Object%20Reference))
  ;[1 1 1] При отключении игрока, проверка на кол-во игроков на сервере
  (bind _asbp_game_instance (Utilities|Casting|CastToBP_GameInstance (Game|GetGameInstance)))
  (Default|OnUnpossess _asbp_game_instance))

(event EventBeginPlay
  (Variables|Default|SetbShowMouseCursor false)
  (Input|SetInputModeGameOnly self)
  ;[1 1 1] Спавним Персонажа
  (bind _asbp_game_instance (Utilities|Casting|CastToBP_GameInstance (Game|GetGameInstance)))
  (Networking|SwitchHasAuthority
    (:Remote
      (CallFunction|SpawnCharacterServer (Variables|/Game/PolygonDungeonOnline/Blueprints/BP_GameInstance.BP_GameInstance_C|GetPlayer%20Character _asbp_game_instance) (Variables|/Game/PolygonDungeonOnline/Blueprints/BP_GameInstance.BP_GameInstance_C|GetCharacter%20Name _asbp_game_instance)))))

(fn ConstructionScript)

(fn GetPlayerCharacter
  (return (.AsBP%20Character%20Base (Utilities|Casting|CastToBP_CharacterBase (Pawn|GetControlledPawn)))))