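; MiniMapCamera is a scene capture camera for the minimap, rendering the world into a runtime-created render target.
; On BeginPlay it creates a small mipmapped texture, stores it as MiniMapTexture and assigns it to the capture component.
; It then hides all Character actors present at that moment from the capture.
; AddHiddenActor lets further actors be excluded individually and prints a leftover debug string.
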(event EventBeginPlay
  (bind _returnvalue (Rendering|CreateRenderTarget2D 300 300 "RTF_RGBA16f" "(R=0.000000,G=0.000000,B=0.000000,A=1.000000)" true))
  (bind _output_get (Variables|Default|SetMiniMap%20Texture _returnvalue))
  (Variables|/Script/Engine.SceneCaptureComponent2D|SetTextureTarget (Variables|DecalActor|GetCaptureComponent2D) _output_get)
  (CallFunction|SetHiddenActors) ; Скрываем ненужные объекты
  (Utilities|Casting|CastToBP_GameInstance (Game|GetGameInstance)))

(fn ConstructionScript)

(fn SetHiddenActors
  (bind _outactors (Actor|GetAllActorsOfClass "/Script/Engine.Character"))
  (Utilities|Array|AppendArray (Variables|/Script/Engine.SceneCaptureComponent|GetHiddenActors (Variables|DecalActor|GetCaptureComponent2D)) _outactors))

(fn AddHiddenActor
  (params (Actor :type Actor%20Object%20Reference))
  (Utilities|Array|AddUnique (Variables|/Script/Engine.SceneCaptureComponent|GetHiddenActors (Variables|DecalActor|GetCaptureComponent2D)) Actor)
  (Development|PrintString "Hello"))