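; BP_GoblinWarior is the Goblin Warrior enemy Blueprint, a thin child class that adds a death-facing rotation.
; Its SetRotationonDeath event takes a rotation and sets the actor's yaw to that yaw minus 180 degrees, zeroing pitch and roll.
; Per the author's note, this turns the goblin opposite to the player who landed the last hit.
; The construction script only calls the parent, and the default BeginPlay, overlap and Tick nodes are disabled.
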(event EventBeginPlay
  (|CallParentFunction) ; This node is disabled and will not be called.\nDrag off pins to build functionality.
)

(event Collision|EventActorBeginOverlap
  (params (OtherActor :type Actor%20Object%20Reference))
  (|CallParentFunction OtherActor) ; This node is disabled and will not be called.\nDrag off pins to build functionality.
)

(event EventTick
  (params (DeltaSeconds :type Float%20%28single-precision%29))
  (|CallParentFunction DeltaSeconds) ; This node is disabled and will not be called.\nDrag off pins to build functionality.
)

(event EventSetRotationonDeath
  (params (Rotation :type Rotator :default "0, 0, 0"))
  ;[1 1 1] Поворот персонажа в противоположную сторону он игрока нанесшего последний удар
  (Transformation|SetActorRotation (Math|Rotator|MakeRotator 0.0 0.0 (- (.Yaw (Math|Rotator|BreakRotator Rotation)) 1.8e+02))))

(fn ConstructionScript
  (|CallParentFunction))