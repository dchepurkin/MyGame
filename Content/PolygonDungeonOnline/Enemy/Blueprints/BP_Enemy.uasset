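; Base enemy Blueprint for a networked game, handling health, damage, death, buffs and aggro modifiers.
; Incoming damage is scaled by shield and damage gain, shown as client-side widgets, and on death triggers multicast montage stop, capsule removal and delayed dissolve.
; Server-spawned buff actors adjust gains, healing and aggro targeting, while RepNotifies broadcast health and buff changes.
; Death rotation is left to child classes, and the aggro accumulation logic is disconnected.
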(event Custom|Stop%20All%20Montages%20Multicast
  (bind (_is_playing_ _current_montage) (Animation|GetMontagePlaying))
  ;[1 1 1] Останавливаем все монтажи
  (if _is_playing_
    (Animation|StopAnimMontage _current_montage)))

(event Custom|Death%20Multicast
  ;[1 0 0] Получение урона
  (Components|DestroyComponent (Variables|Collision|GetCapsuleComponent))
  (CallFunction|RemoveEnemyMulticast))

(event Custom|Apply%20Buff%20Server
  (params (Caster :type Character%20Object%20Reference) (Buff :type BP%20Buff%20Base%20Class%20Reference))
  ;[1 1 1] Активируем баф
  (if (not (Skills|BuffAlreadyCasted? Buff))
    (bind _returnvalue (Game|SpawnActorfromClass Buff (Math|Transform|MakeTransform "0, 0, 0" "0, 0, 0" "1,1,1") "AlwaysSpawn" 0 Caster self 0))
    (Utilities|Array|Add (Variables|Enemy|Skills|GetBuffs) _returnvalue)))

(event Custom|Set%20Rotation%20On%20Death
  (params (Rotation :type Rotator))
  ;[1 0 0] Получение урона
  ;;[1 1 1] Если требуется, то нужно перезаписать в дочернем классе
)

(event Custom|Remove%20Enemy%20Multicast
  ;[1 1 1] Удаление убитого противника
  (Utilities|FlowControl|Delay 3.0)
  (bind _dissolve_amount (Timeline|Dissolve%20Amount PlayFromStart)
    (:Update
      (for _array_element (Actor|GetComponentsbyTag "/Script/Engine.MeshComponent" "Outline")
        (Rendering|Material|SetScalarParameterValueonMaterials _array_element "Dissolve Amount" _dissolve_amount)))
    (:Finished
      (Actor|DestroyActor))))

(event Custom|Play%20Sound%20Multicast
  (params (Sound :type Sound%20Cue%20Object%20Reference))
  ;[1 1 1] Воспроизведение звука
  (Audio|PlaySoundatLocation Sound (Transformation|GetActorLocation) "0, 0, 0" 1.0 1.0 0.0 0 0 0))

(event Custom|Damage%20Widget%20Multicast
  (params (Damage%20Amount :type Float%20%28single-precision%29) (Hill? :type Boolean))
  (bind _returnvalue (Transformation|GetActorLocation))
  ;[1 0 0] Получение урона
  (Networking|SwitchHasAuthority
    (:Remote
      (bind _returnvalue_2 (UserInterface|CreateWidget "/Game/PolygonDungeonOnline/UI/WBP_Damage.WBP_Damage_C" 0 Damage%20Amount Hill? _returnvalue))
      (UserInterface|Viewport|AddtoViewport _returnvalue_2 0)
      (Class|UserWidget|SetPositioninViewport _returnvalue_2 (.ScreenLocation (Class|PlayerController|ProjectWorldLocationtoScreen (Game|GetPlayerController 0) _returnvalue false)) true))))

(event EventApplyDamageGain%
  (params (Input%20Damage%20Gain%25 :type Float%20%28single-precision%29) (Output%20Damage%20Gain :type Float%20%28single-precision%29))
  ;[1 1 1] Активация\отмена бафа на увеличение входящего и исходящего урона
  (Networking|SwitchHasAuthority
    (:Authority
      (Variables|Enemy|Stats|SetInput%20Damage%20Gain%20%25 (+ Input%20Damage%20Gain%25 (Variables|Enemy|Stats|GetInput%20Damage%20Gain%20%25)))
      (Variables|Enemy|Stats|SetOutput%20Damage%20Gain%20%25 (+ (Variables|Enemy|Stats|GetOutput%20Damage%20Gain%20%25) Output%20Damage%20Gain)))))

(event EventRemoveBuff
  (params (Buff :type BP%20Buff%20Base%20Object%20Reference))
  ;[1 1 1] Активируем баф
  (Networking|SwitchHasAuthority
    (:Authority
      (Actor|DestroyActor Buff)
      (Utilities|Array|RemoveItem (Variables|Enemy|Skills|GetBuffs) Buff))))

(event EventCancelAgroGain%
  (params (Argo%20Gain%25 :type Float%20%28single-precision%29) (Agro%20Character :type Character%20Object%20Reference))
  ;[1 1 1] Агро Гейн Баф
  (Utilities|Map|Add (Variables|Enemy|Fight|GetAgro%20Gain%20Table%25) Agro%20Character (- (.Value (Utilities|Map|Find (Variables|Enemy|Fight|GetAgro%20Gain%20Table%25) Agro%20Character)) Argo%20Gain%25)))

(event EventApplyAgroTarget
  (params (Can%20Change%20Target? :type Boolean) (Agro%20Character :type Character%20Object%20Reference))
  ;[1 1 1] Агро Цель
  (bind _output_get (Variables|Enemy|Fight|SetCan%20Change%20Target? Can%20Change%20Target?))
  (if (not _output_get)
    (Variables|Enemy|Fight|SetCurrent%20Target (.AsBP%20Character%20Base (Utilities|Casting|CastToBP_CharacterBase Agro%20Character)))))

(event EventCancelDamageGain%
  (params (Input%20Damage%20Gain%25 :type Float%20%28single-precision%29) (Output%20Damage%20Gain%25 :type Float%20%28single-precision%29))
  ;[1 1 1] Активация\отмена бафа на увеличение входящего и исходящего урона
  (Networking|SwitchHasAuthority
    (:Authority
      (Variables|Enemy|Stats|SetInput%20Damage%20Gain%20%25 (- (Variables|Enemy|Stats|GetInput%20Damage%20Gain%20%25) Input%20Damage%20Gain%25))
      (Variables|Enemy|Stats|SetOutput%20Damage%20Gain%20%25 (- (Variables|Enemy|Stats|GetOutput%20Damage%20Gain%20%25) Output%20Damage%20Gain%25)))))

(event Game|Damage|EventAnyDamage
  (params (Damage :type Float%20%28single-precision%29) (DamageType :type Damage%20Type%20Object%20Reference) (InstigatedBy :type Controller%20Object%20Reference) (DamageCauser :type Actor%20Object%20Reference))
  ;[1 0 0] Получение урона
  (if (not (Variables|Enemy|Stats|GetDead))
    (CallFunction|PlaySoundMulticast (Variables|/Game/PolygonDungeonOnline/Character/Blueprints/BP_CharacterBase.BP_CharacterBase_C|GetHit%20Sound (.AsBP%20Character%20Base (Utilities|Casting|CastToBP_CharacterBase DamageCauser))))
    (bind _dead_ (Fight|GetDamage (* Damage (Variables|Enemy|Stats|GetShield%20Power%20Gain%25))))
    (if _dead_
      (CallFunction|SetRotationonDeath (Transformation|GetActorRotation DamageCauser)) ; Нужно переписывать в дочернем классе
      (CallFunction|DeathMulticast)
      (Skills|RemoveBuffs (Variables|Enemy|Skills|GetBuffs))
      (Default|CallOnDeath))))

(event EventApplyBuff
  (params (Caster :type Character%20Object%20Reference) (Buff :type BP%20Buff%20Base%20Class%20Reference))
  ;[1 1 1] Активируем баф
  (Networking|SwitchHasAuthority
    (:Authority
      (CallFunction|ApplyBuffServer Caster Buff))))

(event EventApplyShieldPowerGain%
  (params (Shield%20Power%20Gain%25 :type Float%20%28single-precision%29))
  ;[1 1 1] Активация\отмена бафа накладываемого щит
  (Networking|SwitchHasAuthority
    (:Authority
      (bind _output_get (Variables|Enemy|Stats|SetShield%20Power%20Gain%25 (- (Variables|Enemy|Stats|GetShield%20Power%20Gain%25) Shield%20Power%20Gain%25)))
      (if (< _output_get 0.0)
        (Variables|Enemy|Stats|SetShield%20Power%20Gain%25 0.0)))))

(event EventCancelShieldPowerGain%
  (params (Shield%20Power%20Gain%25 :type Float%20%28single-precision%29))
  ;[1 1 1] Активация\отмена бафа накладываемого щит
  (Networking|SwitchHasAuthority
    (:Authority
      (bind _output_get (Variables|Enemy|Stats|SetShield%20Power%20Gain%25 (+ (Variables|Enemy|Stats|GetShield%20Power%20Gain%25) Shield%20Power%20Gain%25)))
      (if (> _output_get 1.0)
        (Variables|Enemy|Stats|SetShield%20Power%20Gain%25 1.0)))))

(event EventDOTBuff
  (params (Health%20Res%20DOT :type Float%20%28single-precision%29) (Mana%20Res%20DOT :type Float%20%28single-precision%29) (Stamina%20Res%20DOT :type Float%20%28single-precision%29))
  ;[1 1 1] Дот востановления здоровья
  (Fight|RestoreHealth Health%20Res%20DOT))

(event EventApplyAgroGain%
  (params (Argo%20Gain%25 :type Float%20%28single-precision%29) (Agro%20Character :type Character%20Object%20Reference))
  ;[1 1 1] Агро Гейн Баф
  (Utilities|Map|Add (Variables|Enemy|Fight|GetAgro%20Gain%20Table%25) Agro%20Character (+ Argo%20Gain%25 (.Value (Utilities|Map|Find (Variables|Enemy|Fight|GetAgro%20Gain%20Table%25) Agro%20Character)))))

(fn ConstructionScript)

(fn GetDamage
  (params (Input%20Damage :type Float%20%28single-precision%29))
  (LocalVariables|SetLocal%20Damage (* Input%20Damage (Variables|Enemy|Stats|GetInput%20Damage%20Gain%20%25)))
  (Utilities|FlowControl|Sequence
    (:then_0
      (CallFunction|DamageWidgetMulticast (LocalVariables|GetLocal%20Damage) false))
    (:then_1
      (if (<= (- (Variables|Enemy|Stats|GetCurrent%20Health) (LocalVariables|GetLocal%20Damage)) 0.0)
        (Variables|Enemy|Stats|SetCurrent%20Health 0.0)
        (CallFunction|StopAllMontagesMulticast)
        (Variables|Enemy|Stats|SetDead true)
        (else
          (Variables|Enemy|Stats|SetCurrent%20Health (- (Variables|Enemy|Stats|GetCurrent%20Health) (LocalVariables|GetLocal%20Damage)))))
      (return (Variables|Enemy|Stats|GetDead) (LocalVariables|GetLocal%20Damage)))))

(fn GetMontagePlaying
  (bind _anim_instance (Animation|GetAnimInstance))
  (bind _returnvalue (Animation|Montage|GetCurrentActiveMontage _anim_instance))
  (return (Animation|Montage|MontageIsPlaying _anim_instance _returnvalue) _returnvalue))

(fn GetAnimInstance
  (return (Components|SkeletalMesh|GetAnimInstance (Variables|Character|GetMesh))))

(fn BuffAlreadyCasted?
  (params (Buff :type BP%20Buff%20Base%20Class%20Reference))
  (bind _array_element (Utilities|Array|ForEachLoopwithBreak (Variables|Enemy|Skills|GetBuffs) :!label _label)
    (:LoopBody
      (if (== (Utilities|GetClass _array_element) Buff)
        (LocalVariables|SetLocal%20Bool true)
        (goto _label Break)))
    (:Completed
      (return (LocalVariables|GetLocal%20Bool)))))

(fn RemoveBuffs
  (params (Buffs :type Array%20of%20BP%20Buff%20Base%20Object%20References))
  (for _array_element Buffs
    (Variables|/Game/PolygonDungeonOnline/Blueprints/Skill/BP_Buff_Base.BP_Buff_Base_C|SetCurrent%20Time _array_element 0.0)))

(fn RestoreHealth
  (params (Health :type Float%20%28single-precision%29))
  (bind _output_get (Variables|Enemy|Stats|SetCurrent%20Health (+ Health (Variables|Enemy|Stats|GetCurrent%20Health))))
  (if (>= _output_get (Variables|Enemy|Stats|GetMax%20Health))
    (Variables|Enemy|Stats|SetCurrent%20Health (Variables|Enemy|Stats|GetMax%20Health))))

(fn OnRepBuffs
  (Default|CallOnBuffChanged (Variables|Enemy|Skills|GetBuffs)))

(fn OnRepCurrentHealth
  (Default|CallOnHealthChange (Variables|Enemy|Stats|GetCurrent%20Health) (Variables|Enemy|Stats|GetMax%20Health)))